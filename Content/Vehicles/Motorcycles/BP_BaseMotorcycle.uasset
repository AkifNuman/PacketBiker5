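; Base drivable motorcycle pawn that takes on the entering character's mesh, animation and type flags, and returns possession on exit.
; Self-rescheduling timers drive speed-based FOV, an objective arrow, money sync and fuel drain, showing WB_Win when fuel empties.
; Left Shift triggers character abilities like dash, hover, slow motion or dissolve teleport, using shared macros with cooldowns and some post-process effects.
; High-speed hits eject non-Demon riders into ragdoll.
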(event `InputAxis|Brake`
  (params (AxisValue :type "Float (single-precision)"))
  (`ChaosVehicleMovementComponent.SetBrakeInput` (`self.VehicleMovementComponent`) AxisValue))

(event `InputAxis|Gas`
  (params (AxisValue :type "Float (single-precision)"))
  (bind _fuel (`self.Fuel`))
  (if (`self.InGasStation`)
    (if (<= _fuel 1000.0)
      (set `self.Fuel` (+ _fuel AxisValue)))))

(event `CameraAngles`
  (bind _springarm (`self.SpringArm`))
  (`KismetSystemLibrary.K2_SetTimerDelegate` (delegate `CameraAngles`) 0.033333 true)
  (`CameraComponent.SetFieldOfView` (`self.Camera`) (`KismetMathLibrary.MapRangeClamped` (/ (`ChaosVehicleMovementComponent.GetForwardSpeed` (`self.VehicleMovementComponent`)) 17.0) 0.0 300.0 90.0 110.0))
  (`SceneComponent.K2_SetRelativeRotation` _springarm (`SceneComponent.RelativeRotation` _springarm) false false))

(event `self.EnterBox.OnComponentBeginOverlap`
  (params (OverlappedComponent :type "PrimitiveComponent Object Reference") (OtherActor :type "Actor Object Reference") (OtherComp :type "PrimitiveComponent Object Reference") (OtherBodyIndex :type Integer) (bFromSweep :type Boolean) (SweepResult :type "HitResult Structure (by ref)"))
  (bind _asbp_character (cast `/Game/Characters/BP_Character` OtherActor))
  (set `/Game/Characters/BP_Character.InBox` true _asbp_character)
  (bind _returnvalue (`|CreateWidget` "/Game/Interfaces/Basbana.Basbana_C"))
  (`UserWidget.AddToViewport` _returnvalue 0))

(event `PP`
  (params (Target :type "PostProcessVolume Object Reference") (InBlendableObject :type "BlendableInterface Interface") (InWeight :type "Float (double-precision)"))
  (`PostProcessVolume.AddOrUpdateBlendable` Target InBlendableObject InWeight))

(event `self.EnterBox.OnComponentEndOverlap`
  (params (OverlappedComponent :type "PrimitiveComponent Object Reference") (OtherActor :type "Actor Object Reference") (OtherComp :type "PrimitiveComponent Object Reference") (OtherBodyIndex :type Integer))
  (bind _asbp_character (cast `/Game/Characters/BP_Character` OtherActor))
  (set `/Game/Characters/BP_Character.InBox` false _asbp_character)
  (`Widget.RemoveFromParent` (stale `self.EnterBox.OnComponentBeginOverlap` _returnvalue)))

(event `MakeUnVisible`
  (bind _mesh (`self.Mesh`))
  (bind (_direction _dissolveflot) (`Timeline|Timeline_0` :!label _label)
    (:`Update`
      (`MeshComponent.SetScalarParameterValueOnMaterials` _mesh "Dissolve" _dissolveflot)
      (`MeshComponent.SetScalarParameterValueOnMaterials` _mesh "Dissolve" _dissolveflot)
      (`MeshComponent.SetScalarParameterValueOnMaterials` (`self.Character`) "Dissolve" _dissolveflot))))

(event `MakeRevisible`
  (goto _label :!via `Reverse`))

(event `Key|One`
  (params (Key :type "Key Structure")))

(event `DisableExhaust`
  (params (Condition :type Boolean))
  (`KismetSystemLibrary.Delay` 0.7)
  (if Condition
    (`ActorComponent.Deactivate` (`self.ParticleSystem`))
    (`ActorComponent.Deactivate` (`self.ParticleSystem2`))
    (else
      (`ActorComponent.Activate` (`self.ParticleSystem2`) false)
      (`ActorComponent.Activate` (`self.ParticleSystem`) false))))

(event `SteerCustom`
  (params (Steering :type "Float (double-precision)"))
  ;[1 1 1] BaseControl
  (`ChaosVehicleMovementComponent.SetSteeringInput` (`self.VehicleMovementComponent`) Steering))

(event `InputAxis|Steer`
  (params (AxisValue :type "Float (single-precision)"))
  ;[1 1 1] BaseControl
)

(event `GetInVehicle`
  (params (InputMesh :type "SkeletalMesh Object Reference") (AnimInstance :type "Object Class Reference") (Character :type "Character Object Reference") (AnimInstanceAfterVehicle :type "Object Class Reference") (IsSamurai :type Boolean) (IsGrandma :type Boolean) (IsWizard :type Boolean) (IsGamerGirl :type Boolean) (IsDemon :type Boolean) (IsGrandpa :type Boolean) (IsHomelessMan :type Boolean) (`IsRichFemSci-Fi` :type Boolean))
  (bind _character (`self.Character`))
  (set `self.Char` Character)
  (`self.WhichCharacter` IsSamurai IsGrandma IsWizard IsGamerGirl IsDemon IsGrandpa IsHomelessMan `IsRichFemSci-Fi`)
  (set `self.CharacterAnimClass` AnimInstanceAfterVehicle)
  (`SceneComponent.SetVisibility` (`self.Character`) true false)
  (`self.Activate Movement`)
  (`self.EnableInput` null)
  (bind _outactors (`GameplayStatics.GetAllActorsOfClass` "/Game/Characters/BP_Character.BP_Character_C"))
  (for _array_element _outactors
    (if (`/Game/Characters/BP_Character.HasBox` _array_element)
      (`SceneComponent.SetVisibility` (`/Game/Characters/BP_Character.TasimaKutusu` _array_element) false false)
      (`SceneComponent.SetVisibility` (`self.StaticBox`) true false))
    (set `self.InVehicle` true)
    (`SkinnedMeshComponent.SetSkinnedAssetAndUpdate` _character InputMesh true)
    (`SkeletalMeshComponent.SetAnimInstanceClass` _character AnimInstance)
    (if (`self.IsWizard`)
      (`SceneComponent.K2_SetRelativeLocation` (`self.Character`) (`self.WizzardSeatLoc`) false false)
      (`SceneComponent.SetVisibility` (`self.StaticMesh`) true false))))

(event `DiasableMovement`
  (`PrimitiveComponent.SetConstraintMode` (`self.Mesh`) "XYPlane")
  (`PrimitiveComponent.SetConstraintMode` (`self.Mesh`) "XYPlane")
  (`PrimitiveComponent.SetConstraintMode` (`self.Mesh`) "XYPlane"))

(event `InputAxis|Throttle`
  (params (AxisValue :type "Float (single-precision)")))

(event `Key|LeftShift`
  (params (Key :type "Key Structure"))
  (:`Pressed`
    (if (`self.IsWizard`)
      (`self.Wizard`)
      (elif (`self.IsSamurai`)
        (`self.Samurai_Base`)
        (elif (`self.IsGrandma`)
          (bind _outactors (`GameplayStatics.GetAllActorsOfClass` "/Game/Characters/BP_Grandma.BP_Grandma_C"))
          (for _array_element _outactors
            (`/Game/Characters/BP_Grandma.SpecialForceGrandma` _array_element))
          (elif (`self.IsGrandpa`)
            (`self.Grandpa_Base`)
            (elif (`self.IsRichFemSci-Fi`)
              (`self.Sci-Fi_Base`))))))))

(event `ThrottleCustom`
  (params (Throttle :type "Float (double-precision)"))
  ;[1 1 1] BaseControl
  (`self.DisableExhaust` (> Throttle 0.0))
  (`ChaosVehicleMovementComponent.SetThrottleInput` (`self.VehicleMovementComponent`) Throttle))

(event `self.ReceiveBeginPlay`
  (`|ExecutionSequence`
    (:`then_0`
      (bind _returnvalue (`|CreateWidget` "/Game/Vehicles/Speed.Speed_C"))
      (`UserWidget.AddToViewport` _returnvalue 0)
      (`self.Fueller`))
    (:`then_1`
      (`self.getDolar`))
    (:`then_2`
      (`self.CameraAngles`))
    (:`then_3`
      (`self.arrow2 set directions`))
    (:`then_4`
      (bind _outactors (`GameplayStatics.GetAllActorsOfClassWithTag` "/Script/Engine.PostProcessVolume" "Samurai"))
      (for _array_element _outactors
        (set `self.PostProcess` _array_element)))
    (:`then_5`
      (`self.WizSound`))))

(event `arrow2 set directions`
  (`KismetSystemLibrary.K2_SetTimerDelegate` (delegate `arrow2 set directions`) 0.033333 true)
  (bind _outactors (`GameplayStatics.GetAllActorsOfClass` "/Game/Level_Database/BP_LevelDatabase.Bp_LevelDatabase_C"))
  (for _array_element _outactors
    (if (`/Game/Level_Database/BP_LevelDatabase.isCounter` _array_element)
      (bind _outactors_2 (`GameplayStatics.GetAllActorsOfClass` "/Game/Map/LocationMarker/BP_LocationMarkerRes.BP_LocationMarkerRes_C"))
      (for _array_element_2 _outactors_2
        (`SceneComponent.SetHiddenInGame` (`self.Arrowum`) false false)
        (`SceneComponent.K2_SetWorldRotation` (`self.Arrow`) (`KismetMathLibrary.FindLookAtRotation` (`SceneComponent.K2_GetComponentLocation` (`self.Arrow`)) (`self.K2_GetActorLocation` _array_element_2)) false false))
      (else
        (`SceneComponent.SetHiddenInGame` (`self.Arrowum`) true false)))))

(event `OutOfVehicle`
  (`self.OutOfVehicleFunc`)
  (`self.PP` (`self.PostProcess`) null 0.9)
  (`SceneComponent.SetVisibility` (`self.StaticMesh`) false false)
  (`self.DiasableMovement`))

(event `getDolar`
  (`KismetSystemLibrary.K2_SetTimerDelegate` (delegate `getDolar`) 0.033333 true)
  (bind _outactors (`GameplayStatics.GetAllActorsOfClass` "/Game/Level_Database/BP_LevelDatabase.Bp_LevelDatabase_C"))
  (for _array_element _outactors
    (set `self.Dolar2` (`/Game/Level_Database/BP_LevelDatabase.Dolar` _array_element))))

(event `Up`
  (bind _mesh (`self.Mesh`))
  (`KismetSystemLibrary.PrintString` "UPPPPPPP!!!!!!!" true true (struct :`R` 0.069261 :`B` 1.0 :`A` 1.0))
  (`PrimitiveComponent.SetCenterOfMass` _mesh (-60.0 0.0 -60.0) "None")
  (`KismetSystemLibrary.Delay` 5.0)
  (`PrimitiveComponent.SetCenterOfMass` _mesh (5.0 0.0 -25.0) "None"))

(event `Brake`
  (bind _brakeinput (`self.BrakeInput`))
  (bind _plane1 (`self.Plane1`))
  (bind _mesh (`self.Mesh`))
  (bind (_returnvalue_x _returnvalue_y _returnvalue_z) (`KismetMathLibrary.BreakVector` (`SceneComponent.K2_GetComponentLocation` (`self.Mesh`))))
  (if (> _brakeinput 0.0)
    (`MeshComponent.SetScalarParameterValueOnMaterials` _mesh "LightIntensity" (+ _brakeinput 50.0))
    (if (not (> _returnvalue_z 10.0))
      (`|SpawnActorFromClass` "/Game/Characters/CharacterAbilities/TireTrack/BP_TrackTire.BP_TrackTire_C" (`KismetMathLibrary.MakeTransform` (`SceneComponent.K2_GetComponentLocation` _plane1) (`SceneComponent.K2_GetComponentRotation` _plane1) (0.5 0.5 0.5)) "AlwaysSpawn" "OverrideRootScale" null null)
      (bind _aschopper_bp (cast `/Game/Vehicles/Motorcycles/Chopper/Chopper_BP` (`GameplayStatics.GetPlayerPawn` 0)))
      (`/Game/Vehicles/Motorcycles/Chopper/Chopper_BP.Chopper Track` _aschopper_bp))
    (else
      (`MeshComponent.SetScalarParameterValueOnMaterials` _mesh "LightIntensity" 0.0))))

(event `InputAxis|Brake`
  (params (AxisValue :type "Float (single-precision)")))

(event `Key|T`
  (params (Key :type "Key Structure"))
  (:`Pressed`
    (`self.OutOfVehicle`)))

(event `WizSound`
  (`KismetSystemLibrary.K2_SetTimerDelegate` (delegate `WizSound`) 1.0 true)
  (if (`self.InVehicle`)
    (if (`self.IsWizard`)
      (`GameplayStatics.PlaySoundAtLocation` "/Game/PacketBikerAudio/Wizard/wizard2.wizard2" (`self.K2_GetActorLocation`) (struct) 1.0 1.0 0.0 null null null null))))

(event `Fueller`
  (bind _returnvalue (`KismetMathLibrary.FTrunc` (`ChaosVehicleMovementComponent.GetForwardSpeed` (`self.VehicleMovementComponent`))))
  (`KismetSystemLibrary.K2_SetTimerDelegate` (delegate `Fueller`) 0.016667 true)
  (`/Engine/EditorBlueprintResources/StandardMacros.IsValid` (`GameplayStatics.GetPlayerCharacter` 0)
    (:`Is Not Valid`
      (if (>= _returnvalue 0)
        (set `self.Fuel` (- (`self.Fuel`) (/ (`KismetMathLibrary.Conv_IntToDouble` (+ _returnvalue 10)) 10000.0)))
        (if (<= (`self.Fuel`) 0.0)
          (set `self.Fuel` 0.0)
          (`ActorComponent.Deactivate` (`self.VehicleMovementComponent`))
          (`/Engine/EditorBlueprintResources/StandardMacros.DoOnce` false :!label _label_2
            (:`Completed`
              (bind _returnvalue_2 (`|CreateWidget` "/Game/Fuel/WB_Win.WB_Win_C"))
              (`UserWidget.AddToViewport` _returnvalue_2 0))))
        (else
          (set `self.Fuel` (- (`self.Fuel`) (/ (`KismetMathLibrary.Conv_IntToDouble` (+ 0 10)) 2000.0)))
          (if (<= (`self.Fuel`) 0.0)
            (set `self.Fuel` 0.0)
            (`ActorComponent.Deactivate` (`self.VehicleMovementComponent`))
            (`/Engine/EditorBlueprintResources/StandardMacros.DoOnce` false
              (:`Completed`
                (bind _returnvalue_3 (`|CreateWidget` "/Game/Fuel/WB_Win.WB_Win_C"))
                (`UserWidget.AddToViewport` _returnvalue_3 0)))))))))

(event `ZeroFuel`
  (bind _foundwidgets (`WidgetBlueprintLibrary.GetAllWidgetsOfClass` "/Game/Fuel/WB_Win.WB_Win_C"))
  (`Widget.RemoveFromParent` _foundwidgets)
  (if (!= (`self.Dolar2`) 0)
    (goto _label_2 :!via `Reset`)))

(event `self.Box.OnComponentBeginOverlap`
  (params (OverlappedComponent :type "PrimitiveComponent Object Reference") (OtherActor :type "Actor Object Reference") (OtherComp :type "PrimitiveComponent Object Reference") (OtherBodyIndex :type Integer) (bFromSweep :type Boolean) (SweepResult :type "HitResult Structure (by ref)"))
  (bind _returnvalue (`GameplayStatics.GetObjectClass` OtherActor))
  (`/Engine/EditorBlueprintResources/StandardMacros.DoOnce` false :!label _label_3
    (:`Completed`
      (if (`self.InVehicle`)
        (if (`self.IsDemon`)
          _
          (elif (or (or (== _returnvalue null) (== _returnvalue "/Game/Characters/BP_Character.BP_Character_C")) (or (== _returnvalue null) (== _returnvalue null)))
            (if (> (`ChaosVehicleMovementComponent.GetForwardSpeed` (`self.VehicleMovementComponent`)) 750.0)
              (`self.OutOfVehicle`)
              (bind _asbp_character (cast `/Game/Characters/BP_Character` (`GameplayStatics.GetPlayerPawn` 0)))
              (`/Game/Characters/BP_Character.Ragdoll` _asbp_character))))))))

(event `self.Box.OnComponentEndOverlap`
  (params (OverlappedComponent :type "PrimitiveComponent Object Reference") (OtherActor :type "Actor Object Reference") (OtherComp :type "PrimitiveComponent Object Reference") (OtherBodyIndex :type Integer))
  (`KismetSystemLibrary.Delay` 10.0)
  (goto _label_3 :!via `Reset`))

(fn `Activate Movement`
  (`PrimitiveComponent.SetConstraintMode` (`self.Mesh`) "None")
  (`PrimitiveComponent.SetConstraintMode` (`self.Mesh`) "None"))

(fn `CarFlip`
  (bind (_returnvalue_roll _returnvalue_pitch _returnvalue_yaw) (`KismetMathLibrary.BreakRotator` (`self.K2_GetActorRotation`)))
  (bind _returnvalue (`self.K2_GetActorLocation`))
  (if (< (`KismetMathLibrary.VSize` (`self.GetVelocity`)) 20.0)
    (bind _returnvalue_2 (`self.K2_TeleportTo` (+ _returnvalue (0.0 0.0 100.0)) (`KismetMathLibrary.MakeRotator` 0.0 0.0 _returnvalue_yaw)))
    (if _returnvalue_2
      (`KismetSystemLibrary.PrintString` "Flipliyo Abi")
      (else
        (bind _returnvalue_3 (`self.K2_TeleportTo` (+ _returnvalue (0.0 0.0 200.0)) (`KismetMathLibrary.MakeRotator` 0.0 0.0 _returnvalue_yaw)))
        (if (not _returnvalue_3)
          (bind _returnvalue_4 (`self.K2_TeleportTo` (+ _returnvalue (100.0 0.0 100.0)) (`KismetMathLibrary.MakeRotator` 0.0 0.0 _returnvalue_yaw)))
          (if (not _returnvalue_4)
            (`self.K2_TeleportTo` (+ _returnvalue (0.0 0.0 1000.0)))
            (`KismetSystemLibrary.PrintString` "YARRAAAAAAAAAAAA")))))))

(fn `MySteer`
  (params (Steering1 :type "Float (double-precision)")))

(fn `OutOfVehicleFunc`
  (bind _staticbox (`self.StaticBox`))
  (`self.Activate Movement`)
  (set `self.InVehicle` false)
  (bind _outactors (`GameplayStatics.GetAllActorsOfClass` "/Game/Characters/BP_Character.BP_Character_C"))
  (for _array_element _outactors
    (`self.DisableInput` null)
    (`SceneComponent.SetVisibility` (`Character.Mesh` _array_element) true false)
    (`self.SetActorEnableCollision` _array_element true)
    (if (`/Game/Characters/BP_Character.HasBox` _array_element)
      (`SceneComponent.SetVisibility` (`/Game/Characters/BP_Character.TasimaKutusu` _array_element) true false)
      (`SceneComponent.SetVisibility` _staticbox false false)
      (else
        (`SceneComponent.SetVisibility` _staticbox false false)
        (`SceneComponent.SetVisibility` (`/Game/Characters/BP_Character.TasimaKutusu` _array_element) false false)))
    (bind _returnvalue (`self.K2_TeleportTo` :`self` _array_element :`DestLocation` (`SceneComponent.K2_GetComponentLocation` (`self.OutOf`))))
    (if (not _returnvalue)
      (`KismetSystemLibrary.PrintString` (`KismetStringLibrary.Conv_BoolToString` _returnvalue))
      (`self.K2_TeleportTo` :`self` _array_element :`DestLocation` (`SceneComponent.K2_GetComponentLocation` (`self.OutOfOtherSide`))))
    (`Controller.Possess` (`GameplayStatics.GetPlayerController` 0) _array_element)
    (`SkinnedMeshComponent.SetSkinnedAssetAndUpdate` (`self.Character`) null true)))

(fn `UserConstructionScript`
  (`parent.UserConstructionScript`))