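; Chopper motorcycle Blueprint that adds per-character special abilities, a Space-bar flip and tire-track spawning to its parent vehicle.
; Ability events call macros for Wizard and Samurai forward boosts, Grandpa slow motion, Grandma post-process toggling and a sci-fi dissolve-and-teleport.
; Each macro gates reuse with DoOnce and Delay cooldowns.
; Cel-shader post-process blendables and a Dissolve timeline on mesh and rider materials drive several effects.
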(event `Chopper Track`
  (`|SpawnActorFromClass` "/Game/Characters/CharacterAbilities/TireTrack/BP_TrackTire.BP_TrackTire_C" (`SceneComponent.K2_GetComponentToWorld` (`self.Plane2`)) "AlwaysSpawn" "OverrideRootScale" null null))

(event `self.ReceiveBeginPlay`
  (`parent.ReceiveBeginPlay`)
  (set `self.WizzardSeatLoc` (-67.646123 0.0 76.040425)))

(event `Key|SpaceBar`
  (params (Key :type "Key Structure"))
  (:`Pressed`
    (`self.CarFlip`)))

(event `DiasableMovement`
  (bind _mesh (`self.Mesh`))
  (`PrimitiveComponent.SetConstraintMode` _mesh "XYPlane")
  (`PrimitiveComponent.SetConstraintMode` _mesh "XYPlane"))

(event `MakeUnVisible`
  (bind _mesh (`self.Mesh`))
  (bind (_direction _dissolveflot) (`Timeline|Dissolving` :!label _label)
    (:`Update`
      (`MeshComponent.SetScalarParameterValueOnMaterials` _mesh "Dissolve" _dissolveflot)
      (`MeshComponent.SetScalarParameterValueOnMaterials` _mesh "Dissolve" _dissolveflot)
      (`MeshComponent.SetScalarParameterValueOnMaterials` (`self.Character`) "Dissolve" _dissolveflot))))

(event `MakeRevisible`
  (goto _label :!via `Reverse`))

(event `GrandmaDefaultVi`)

(event `WizzardAbility`
  (`self.Wizard`))

(event `GrandmaAbility`
  (`self.Grandma` null))

(event `GrandpaAbility`
  (`self.Grandpa`))

(event `SamuraiAbility`
  (`self.Samurai`))

(event `RichFemSci-Fi_AbilityScooter`
  (`self.RichFemSci-Fi`))

(fn `UserConstructionScript`
  (`parent.UserConstructionScript`))