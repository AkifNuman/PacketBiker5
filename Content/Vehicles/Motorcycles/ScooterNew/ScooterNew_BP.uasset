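; Player scooter vehicle Blueprint with per-rider special abilities, each gated by a DoOnce that resets after delayed cooldowns.
; Tick feeds forward speed to engine audio as RPM, and Space triggers CarFlip.
; Ability events call macros: Grandma toggles post-process, Grandpa slows time under a newsprint shader, Samurai dashes, RichFemSciFi dissolves and teleports forward via a timeline.
; A Wizard boost with steam exists, but its event is empty.
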(event `self.ReceiveBeginPlay`
  (`parent.ReceiveBeginPlay`)
  (set `self.WizzardSeatLoc` (-32.0 0.0 80.741607)))

(event `self.ReceiveTick`
  (params (DeltaSeconds :type "Float (single-precision)"))
  (`AudioComponent.SetFloatParameter` (`self.ScooterNewEnginecube`) "RPM" (`KismetMathLibrary.Abs` (`ChaosVehicleMovementComponent.GetForwardSpeed` (`self.VehicleMovementComponent`))))
  (`KismetSystemLibrary.PrintString` (`KismetStringLibrary.Conv_BoolToString` (`self.IsWizard`))))

(event `Key|SpaceBar`
  (params (Key :type "Key Structure"))
  (:`Pressed`
    (`self.CarFlip`)))

(event `DiasableMovement`
  (bind _mesh (`self.Mesh`))
  (`PrimitiveComponent.SetConstraintMode` _mesh "XYPlane")
  (`PrimitiveComponent.SetConstraintMode` _mesh "XYPlane"))

(event `MakeUnVisible`
  (bind _mesh (`self.Mesh`))
  (bind (_direction _dissolveflot) (`Timeline|Dissolving` :!label _label)
    (:`Update`
      (`MeshComponent.SetScalarParameterValueOnMaterials` _mesh "Dissolve" _dissolveflot)
      (`MeshComponent.SetScalarParameterValueOnMaterials` _mesh "Dissolve" _dissolveflot)
      (`MeshComponent.SetScalarParameterValueOnMaterials` (`self.Character`) "Dissolve" _dissolveflot))))

(event `MakeRevisible`
  (goto _label :!via `Reverse`))

(event `GrandmaDefaultVi`)

(event `WizzardAbility`)

(event `GrandmaAbility`
  (`self.Grandma` null))

(event `GrandpaAbility`
  (`self.Grandpa`))

(event `SamuraiAbility`
  (`self.Samurai`))

(event `RichFemSci-Fi_AbilityScooter`
  (`self.RichFemSci-Fi`))

(fn `UserConstructionScript`
  (`parent.UserConstructionScript`))