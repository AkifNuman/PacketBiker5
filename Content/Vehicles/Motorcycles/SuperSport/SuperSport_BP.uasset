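; SuperSport motorcycle Blueprint with rider-specific abilities, a spacebar flip and timeline-driven dissolve of bike and rider.
; Tick feeds forward speed into the engine's RPM parameter and draws a center-of-mass debug sphere.
; Ability events call cooldown-gated graphs: Grandma temporarily clears a post-process blendable, Grandpa slows global time while speeding up the bike under a newsprint shader, Samurai boosts forward.
; Wizard's boost graph exists, but its event is empty.
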(event `self.ReceiveTick`
  (params (DeltaSeconds :type "Float (single-precision)"))
  (`AudioComponent.SetFloatParameter` (`self.SuperSportEnginecube`) "RPM" (`KismetMathLibrary.Abs` (`ChaosVehicleMovementComponent.GetForwardSpeed` (`self.VehicleMovementComponent`))))
  (`KismetSystemLibrary.DrawDebugSphere` (`PrimitiveComponent.GetCenterOfMass` (`self.Mesh`) "None") 25.0 12 (struct :`R` 1.0 :`B` 0.75 :`A` 1.0)))

(event `Key|SpaceBar`
  (params (Key :type "Key Structure"))
  (:`Pressed`
    (`self.CarFlip`)))

(event `DiasableMovement`
  (bind _mesh (`self.Mesh`))
  (`PrimitiveComponent.SetConstraintMode` _mesh "XYPlane")
  (`PrimitiveComponent.SetConstraintMode` _mesh "XYPlane"))

(event `MakeUnVisible`
  (bind _mesh (`self.Mesh`))
  (bind (_direction _dissolveflot) (`Timeline|Dissolving` :!label _label)
    (:`Update`
      (`MeshComponent.SetScalarParameterValueOnMaterials` _mesh "Dissolve" _dissolveflot)
      (`MeshComponent.SetScalarParameterValueOnMaterials` _mesh "Dissolve" _dissolveflot)
      (`MeshComponent.SetScalarParameterValueOnMaterials` (`self.Character`) "Dissolve" _dissolveflot))))

(event `MakeRevisible`
  (goto _label :!via `Reverse`))

(event `GrandmaDefaultVi`)

(event `WizzardAbility`)

(event `GrandmaAbility`
  (`self.Grandma` null))

(event `GrandpaAbility`
  (`self.Grandpa`))

(event `SamuraiAbility`
  (`self.Samurai`))

(event `RichFemSci-Fi_AbilityScooter`)

(fn `UserConstructionScript`
  (`parent.UserConstructionScript`))