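; Bobber motorcycle Blueprint with character-specific abilities and a Space-key car flip.
; Ability events trigger macros that cool down via DoOnce and delays: Grandma post-process toggle, Grandpa slow motion, Samurai forward dash, and RichFemSci-Fi dissolve-teleport.
; Cel-shader post-process blendables restyle the view, while a timeline drives material dissolve for the teleport.
; The Wizard boost and Grandma default-view graphs exist, but their events are empty.
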(event `self.ReceiveTick`
  (params (DeltaSeconds :type "Float (single-precision)")))

(event `Key|SpaceBar`
  (params (Key :type "Key Structure"))
  (:`Pressed`
    (`self.CarFlip`)))

(event `DiasableMovement`
  (bind _mesh (`self.Mesh`))
  (`PrimitiveComponent.SetConstraintMode` _mesh "XYPlane")
  (`PrimitiveComponent.SetConstraintMode` _mesh "XYPlane"))

(event `MakeUnVisible`
  (bind _mesh (`self.Mesh`))
  (bind (_direction _dissolveflot) (`Timeline|Dissolving` :!label _label)
    (:`Update`
      (`MeshComponent.SetScalarParameterValueOnMaterials` _mesh "Dissolve" _dissolveflot)
      (`MeshComponent.SetScalarParameterValueOnMaterials` _mesh "Dissolve" _dissolveflot)
      (`MeshComponent.SetScalarParameterValueOnMaterials` (`self.Character`) "Dissolve" _dissolveflot))))

(event `MakeRevisible`
  (goto _label :!via `Reverse`))

(event `GrandmaDefaultVi`)

(event `WizzardAbility`)

(event `GrandmaAbility`
  (`self.Grandma` null))

(event `GrandpaAbility`
  (`self.Grandpa`))

(event `SamuraiAbility`
  (`self.Samurai`))

(event `RichFemSci-Fi_AbilityScooter`
  (`self.RichFemSci-Fi`))

(fn `UserConstructionScript`
  (`parent.UserConstructionScript`))