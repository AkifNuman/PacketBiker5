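; BP_RestaurantPoint is a spinning restaurant pickup point for a delivery mission.
; When the player overlaps its box and its number matches a BP_TargetCalculator's restaurant location, it destroys the current location marker.
; It then finds target points matching the calculator's target, gives the player a visible carry box, reveals the destination, spawns a marker there and hides itself.
; Lookups use nested class-wide actor searches, with debug prints along the way.
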(event `self.ReceiveTick`
  (params (DeltaSeconds :type "Float (single-precision)"))
  (bind (_returnvalue_roll _returnvalue_pitch _returnvalue_yaw) (`KismetMathLibrary.BreakRotator` (`self.K2_GetActorRotation`)))
  (`self.K2_SetActorRotation` (`KismetMathLibrary.MakeRotator` _returnvalue_roll _returnvalue_pitch (+ _returnvalue_yaw 1.0))))

(event `self.Box.OnComponentBeginOverlap`
  (params (OverlappedComponent :type "PrimitiveComponent Object Reference") (OtherActor :type "Actor Object Reference") (OtherComp :type "PrimitiveComponent Object Reference") (OtherBodyIndex :type Integer) (bFromSweep :type Boolean) (SweepResult :type "HitResult Structure (by ref)"))
  (bind _returnvalue (`GameplayStatics.GetPlayerCharacter` 0))
  (`/Engine/EditorBlueprintResources/StandardMacros.IsValid` _returnvalue
    (:`Is Valid`
      (if (== OtherActor _returnvalue)
        (bind _outactors (`GameplayStatics.GetAllActorsOfClass` "/Game/Mission/BP_TargetCalculator.BP_TargetCalculator_C"))
        (for _array_element _outactors
          (if (== (`self.RestauranNumber`) (`/Game/Mission/BP_TargetCalculator.ResLoc` _array_element))
            (bind _returnvalue_2 (`GameplayStatics.GetActorOfClass` "/Game/Map/LocationMarker/BP_LocationMarkerRes.BP_LocationMarkerRes_C"))
            (`self.K2_DestroyActor` _returnvalue_2)
            (bind _outactors_2 (`GameplayStatics.GetAllActorsOfClass` "/Game/Mission/BP_TargetCalculator.BP_TargetCalculator_C"))
            (for _array_element_2 _outactors_2
              (bind _tarloc (`/Game/Mission/BP_TargetCalculator.TarLoc` _array_element_2))
              (`KismetSystemLibrary.PrintString` (`KismetStringLibrary.Conv_IntToString` _tarloc))
              (bind _outactors_3 (`GameplayStatics.GetAllActorsOfClass` "/Game/Mission/BP_TargetPoint.BP_TargetPoint_C"))
              (for _array_element_3 _outactors_3
                (if (== (`/Game/Mission/BP_TargetPoint.Target Number` _array_element_3) _tarloc)
                  (bind _asbp_character (cast `/Game/Characters/BP_Character` (`GameplayStatics.GetPlayerPawn` 0)))
                  (set `/Game/Characters/BP_Character.HasBox` true _asbp_character)
                  (`SceneComponent.SetVisibility` (`/Game/Characters/BP_Character.TasimaKutusu` _asbp_character) true false)
                  (`self.SetActorHiddenInGame` _array_element_3 false)
                  (bind _returnvalue_3 (`self.GetTransform` _array_element_3))
                  (`KismetSystemLibrary.PrintString` (`KismetStringLibrary.Conv_TransformToString` _returnvalue_3))
                  (`|SpawnActorFromClass` "/Game/Map/LocationMarker/BP_LocationMarkerRes.BP_LocationMarkerRes_C" _returnvalue_3 "AlwaysSpawn" "OverrideRootScale" null null)
                  (`self.SetActorHiddenInGame` true))))))))))

(fn `UserConstructionScript`)