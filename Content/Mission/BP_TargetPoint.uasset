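; BP_TargetPoint is a spinning delivery point that completes a box-carrying mission when the player overlaps it.
; If a BP_TargetCalculator's TarLoc matches its TargetNumber, it clears the character's box and destroys the location marker and calculators.
; It pays Dolar into Bp_LevelDatabase, adding a bonus and sound for any remaining MissionCounter.
; Nested GetAllActorsOfClass loops also remove the counter and widget, then hide the point.
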(event `self.ReceiveTick`
  (params (DeltaSeconds :type "Float (single-precision)"))
  (bind (_returnvalue_roll _returnvalue_pitch _returnvalue_yaw) (`KismetMathLibrary.BreakRotator` (`self.K2_GetActorRotation`)))
  (`self.K2_SetActorRotation` (`KismetMathLibrary.MakeRotator` _returnvalue_roll _returnvalue_pitch (+ _returnvalue_yaw 1.0))))

(event `self.Box.OnComponentBeginOverlap`
  (params (OverlappedComponent :type "PrimitiveComponent Object Reference") (OtherActor :type "Actor Object Reference") (OtherComp :type "PrimitiveComponent Object Reference") (OtherBodyIndex :type Integer) (bFromSweep :type Boolean) (SweepResult :type "HitResult Structure (by ref)"))
  (bind _returnvalue (`GameplayStatics.GetPlayerCharacter` 0))
  (`/Engine/EditorBlueprintResources/StandardMacros.IsValid` _returnvalue
    (:`Is Valid`
      (if (== OtherActor _returnvalue)
        (bind _outactors (`GameplayStatics.GetAllActorsOfClass` "/Game/Mission/BP_TargetCalculator.BP_TargetCalculator_C"))
        (for _array_element _outactors
          (if (== (`/Game/Mission/BP_TargetCalculator.TarLoc` _array_element) (`self.Target Number`))
            (bind _asbp_character (cast `/Game/Characters/BP_Character` _returnvalue))
            (set `/Game/Characters/BP_Character.HasBox` false _asbp_character)
            (`SceneComponent.SetVisibility` (`/Game/Characters/BP_Character.TasimaKutusu` _asbp_character) false false)
            (bind _returnvalue_2 (`GameplayStatics.GetActorOfClass` "/Game/Map/LocationMarker/BP_LocationMarkerRes.BP_LocationMarkerRes_C"))
            (`self.K2_DestroyActor` _returnvalue_2)
            (bind _outactors_2 (`GameplayStatics.GetAllActorsOfClass` "/Game/Mission/BP_TargetCalculator.BP_TargetCalculator_C"))
            (for _array_element_2 _outactors_2
              (`self.K2_DestroyActor` _array_element_2)
              (bind _outactors_3 (`GameplayStatics.GetAllActorsOfClass` "/Game/Level_Database/BP_LevelDatabase.Bp_LevelDatabase_C"))
              (for _array_element_3 _outactors_3
                (set `/Game/Level_Database/BP_LevelDatabase.Dolar` (+ (`/Game/Level_Database/BP_LevelDatabase.Dolar` _array_element_3) 5) _array_element_3)
                (set `/Game/Level_Database/BP_LevelDatabase.isCounter` false _array_element_3)
                (bind _outactors_4 (`GameplayStatics.GetAllActorsOfClass` "/Game/Level_Database/Counter/BP_Counter.BP_Counter_C"))
                (for _array_element_4 _outactors_4
                  (bind _missioncounter (`/Game/Level_Database/Counter/BP_Counter.MissionCounter` _array_element_4))
                  (if (> _missioncounter 0)
                    (`GameplayStatics.PlaySoundAtLocation` "/Game/PacketBikerAudio/MissionComplete/cash-register-purchase-87313.cash-register-purchase-87313" (`self.K2_GetActorLocation` (`GameplayStatics.GetPlayerPawn` 0)) (struct) 1.0 1.0 0.0 null null null)
                    (set `/Game/Level_Database/BP_LevelDatabase.Dolar` (+ (`/Game/Level_Database/BP_LevelDatabase.Dolar` _array_element_3) (/ _missioncounter 10)) _array_element_3))
                  (`self.K2_DestroyActor` _array_element_4)
                  (bind _foundwidgets (`WidgetBlueprintLibrary.GetAllWidgetsOfClass` "/Game/Level_Database/WB_MissionCounter.WB_MissionCounter_C"))
                  (for _array_element_5 _foundwidgets
                    (`Widget.RemoveFromParent` _array_element_5)
                    (`self.SetActorHiddenInGame` true)))))))))))

(fn `UserConstructionScript`)