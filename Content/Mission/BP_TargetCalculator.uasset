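; Mission setup actor that picks a random restaurant and delivery target on BeginPlay and sizes the mission counter from the trip distance.
; It reveals the chosen BP_RestaurantPoint and spawns a location marker and BP_Counter there.
; Helpers measure metres from the player character, or a BP_BaseMotorcycle if no character is valid, to the restaurant, then restaurant to target.
; Their sum divided by five sets every counter's current and maximum values.
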(event `self.ReceiveBeginPlay`
  (bind _output_get (set `self.ResLoc` (`KismetMathLibrary.RandomIntegerInRange` 0 (`self.MaxRes`))))
  (`KismetSystemLibrary.PrintString` (`KismetStringLibrary.Conv_IntToString` _output_get))
  (bind _output_get_2 (set `self.TarLoc` (`KismetMathLibrary.RandomIntegerInRange` 0 (`self.MaxTar`))))
  (`KismetSystemLibrary.PrintString` (`KismetStringLibrary.Conv_IntToString` _output_get_2))
  (bind _outactors (`GameplayStatics.GetAllActorsOfClass` "/Game/Mission/BP_RestaurantPoint.BP_RestaurantPoint_C"))
  (for _array_element _outactors
    (if (== (`/Game/Mission/BP_RestaurantPoint.RestauranNumber` _array_element) (`self.ResLoc`))
      (`self.SetActorHiddenInGame` _array_element false)
      (bind _returnvalue (`self.GetTransform` _array_element))
      (`|SpawnActorFromClass` "/Game/Map/LocationMarker/BP_LocationMarkerRes.BP_LocationMarkerRes_C" _returnvalue "AlwaysSpawn" "OverrideRootScale" null null)
      (`|SpawnActorFromClass` "/Game/Level_Database/Counter/BP_Counter.BP_Counter_C" _returnvalue "AlwaysSpawn" "OverrideRootScale" null null)
      (`/Engine/EditorBlueprintResources/StandardMacros.IsValid` (`GameplayStatics.GetPlayerCharacter` 0)
        (:`Is Valid`
          (bind _outactors_2 (`GameplayStatics.GetAllActorsOfClass` "/Game/Mission/BP_RestaurantPoint.BP_RestaurantPoint_C"))
          (for _array_element_2 _outactors_2
            (if (== (`/Game/Mission/BP_RestaurantPoint.RestauranNumber` _array_element_2) (`self.ResLoc`))
              (`|ExecutionSequence`
                (:`then_0`
                  (bind _returnvalue_2 (`self.WithCharacter` (`self.K2_GetActorLocation` _array_element_2)))
                  (bind _outactors_3 (`GameplayStatics.GetAllActorsOfClass` "/Game/Level_Database/Counter/BP_Counter.BP_Counter_C"))
                  (for _array_element_3 _outactors_3
                    (bind _returnvalue_3 (/ (+ _returnvalue_2 (stale _newparam)) 5))
                    (set `/Game/Level_Database/Counter/BP_Counter.MissionCounter` _returnvalue_3 _array_element_3 :!label _label)
                    (set `/Game/Level_Database/Counter/BP_Counter.MaxMissionCounter` _returnvalue_3 _array_element_3)))
                (:`then_1`
                  (bind _newparam (`self.ResDistancetoTar`))
                  (goto _label))))))
        (:`Is Not Valid`
          (bind _outactors_4 (`GameplayStatics.GetAllActorsOfClass` "/Game/Mission/BP_RestaurantPoint.BP_RestaurantPoint_C"))
          (for _array_element_4 _outactors_4
            (if (== (`/Game/Mission/BP_RestaurantPoint.RestauranNumber` _array_element_4) (`self.ResLoc`))
              (`|ExecutionSequence`
                (:`then_0`
                  (bind _newparam1 (`self.WithScooter` (`self.K2_GetActorLocation` _array_element_4)))
                  (bind _outactors_5 (`GameplayStatics.GetAllActorsOfClass` "/Game/Level_Database/Counter/BP_Counter.BP_Counter_C"))
                  (for _array_element_5 _outactors_5
                    (bind _returnvalue_4 (/ (+ _newparam1 (stale _newparam_2)) 5))
                    (set `/Game/Level_Database/Counter/BP_Counter.MissionCounter` _returnvalue_4 _array_element_5 :!label _label_2)
                    (set `/Game/Level_Database/Counter/BP_Counter.MaxMissionCounter` _returnvalue_4 _array_element_5)))
                (:`then_1`
                  (bind _newparam_2 (`self.ResDistancetoTar`))
                  (goto _label_2))))))))))

(fn `ResDistancetoTar`
  (returns (NewParam :type Integer))
  (bind _outactors (`GameplayStatics.GetAllActorsOfClass` "/Game/Mission/BP_RestaurantPoint.BP_RestaurantPoint_C"))
  (for _array_element _outactors
    (if (== (`/Game/Mission/BP_RestaurantPoint.RestauranNumber` _array_element) (`self.ResLoc`))
      (bind _outactors_2 (`GameplayStatics.GetAllActorsOfClass` "/Game/Mission/BP_TargetPoint.BP_TargetPoint_C"))
      (for _array_element_2 _outactors_2
        (if (== (`self.TarLoc`) (`/Game/Mission/BP_TargetPoint.Target Number` _array_element_2))
          (bind _returnvalue (`KismetMathLibrary.Vector_Distance` (`self.K2_GetActorLocation` _array_element) (`self.K2_GetActorLocation` _array_element_2)))
          (`KismetSystemLibrary.PrintString` (`KismetStringLibrary.Concat_StrStr` (`KismetStringLibrary.Conv_DoubleToString` _returnvalue) " res + tar"))
          (return (`KismetMathLibrary.FTrunc` (/ _returnvalue 100.0))))))))

(fn `UserConstructionScript`)

(fn `WithCharacter`
  (params (NewParam :type "Vector Structure"))
  (returns (ReturnValue :type Integer))
  (return (`KismetMathLibrary.FTrunc` (/ (`KismetMathLibrary.Vector_Distance` (`self.K2_GetActorLocation` (`GameplayStatics.GetPlayerCharacter` 0)) NewParam) 100.0))))

(fn `WithScooter`
  (params (actorlocation :type "Vector Structure"))
  (returns (NewParam1 :type Integer))
  (bind _outactors (`GameplayStatics.GetAllActorsOfClass` "/Game/Vehicles/Motorcycles/BP_BaseMotorcycle.BP_BaseMotorcycle_C"))
  (for _array_element _outactors
    (bind _returnvalue (`KismetMathLibrary.FTrunc` (/ (`KismetMathLibrary.Vector_Distance` (`self.K2_GetActorLocation` _array_element) actorlocation) 100.0)))
    (`KismetSystemLibrary.PrintString` (`KismetStringLibrary.Concat_StrStr` (`KismetStringLibrary.Conv_IntToString` _returnvalue) "mot + res"))
    (return _returnvalue)))