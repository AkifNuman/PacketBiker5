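; Server-side traffic spawner that populates BP_SplineRoad splines with BP_BaseVehicleParent vehicles.
; BeginPlay gathers eligible roads, either flagged custom ones or long non-highway splines, then starts a looping timer.
; Each tick picks a random road, box-traces near the spline origin for blockage, spawns either random or per-class quota vehicles and passes them spawner settings.
; Optional respawning periodically rechecks the count against MaxVehicle and resumes random spawning.
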(event `self.ReceiveBeginPlay`
  ;[1 1 1] Get alla spline on map
  (`/Engine/EditorBlueprintResources/ActorMacros.Switch Has Authority`
    (:`Authority`
      (`KismetArrayLibrary.Array_Clear` (`self.ArraySpline`))
      (bind _outactors (`GameplayStatics.GetAllActorsOfClass` "/Game/TrafficSystem/BP_SplineRoad.BP_SplineRoad_C"))
      (set `self.AllSplineArray` _outactors)
      (if (`self.CustomSpawn?`)
        ;;[1 1 1] if you want spawn vehicle on specific spline
        (for _array_element (`self.AllSplineArray`)
          (if (`/Game/TrafficSystem/BP_SplineRoad.SpawnOnThisSpine?` _array_element)
            (`KismetArrayLibrary.Array_Add` (`self.ArraySpline`) _array_element)))
        (`self.StartTimer`)
        (else
          ;;[1 1 1] Spawn on all spline
          (for _array_element_2 (`self.AllSplineArray`)
            (bind _highspeedroad (`/Game/TrafficSystem/BP_SplineRoad.HighSpeedRoad` _array_element_2))
            (if (and (not _highspeedroad) (>= (`SplineComponent.GetSplineLength` (`/Game/TrafficSystem/BP_SplineRoad.Spline` _array_element_2)) 1500.0))
              (`KismetArrayLibrary.Array_Add` (`self.ArraySpline`) _array_element_2)
              (elif _highspeedroad
                (`KismetArrayLibrary.Array_Add` (`self.ArraySplineHighway`) _array_element_2))))
          (`self.StartTimer`))))))

(event `StartTimer`
  ;[1 1 1] Start Timer to spawn vehicle
  (if (`self.VehicleNumPerClass`)
    (bind _returnvalue (`KismetSystemLibrary.K2_SetTimer` null "CheckAndSpawnPerClass" (select `bool` (`self.TimeBetweenSpawn`) :`false` 0.1 :`true` (`KismetMathLibrary.RandomFloatInRange` (`self.MinTimeBetweenSpawn`) (`self.MaxTimeBetweenSpawn`))) true))
    (set `self.TimerHandle` _returnvalue)
    (else
      (bind _returnvalue_2 (`KismetSystemLibrary.K2_SetTimer` null "SpawnRandom" 0.1 true))
      (set `self.TimerHandle` _returnvalue_2))))

(event `SpawnRandom`
  ;[1 1 1] Random spawn event
  (if (< (`KismetArrayLibrary.Array_Length` (`self.SpawnedVehicleArray`)) (`self.MaxVehicle`))
    (if (`self.TimeBetweenSpawn`)
      (`KismetSystemLibrary.Delay` (`KismetMathLibrary.RandomFloatInRange` (`self.MinTimeBetweenSpawn`) (`self.MaxTimeBetweenSpawn`)))
      (`self.CheckAndSpawn`)
      (else
        (`self.CheckAndSpawn`)))
    (else
      ;[1 1 1] Once all vehicles have spawned, pause the Timer and check whether to continue spawning or stopping, depending on the settings
      (`KismetSystemLibrary.K2_PauseTimerHandle` (`self.TimerHandle`))
      (`KismetSystemLibrary.K2_SetTimer` null "ContinueSpawn" 30.0))))

(fn `CheckAndSpawn`
  (locals (RandomPointOnSpline :type Integer))
  (bind _spline (`/Game/TrafficSystem/BP_SplineRoad.Spline` (`self.Spline`)))
  (bind (_returnvalue_x _returnvalue_y _returnvalue_z) (`KismetMathLibrary.BreakVector` (`SplineComponent.GetLocationAtSplinePoint` _spline 0 "World")))
  ;[1 1 1] Spawn vehicles and set spawner settings in vehicles
  (set `self.RandomInt` (`KismetMathLibrary.RandomIntegerInRange` 0 (`KismetArrayLibrary.Array_LastIndex` (`self.ArraySpline`))))
  (bind (_output _colliding_) (`self.CheckCollision`))
  (set `self.Spline` _output)
  (if (not _colliding_)
    (set `local.RandomPointOnSpline` (`KismetMathLibrary.RandomInteger` (- (`SplineComponent.GetNumberOfSplinePoints` _spline) 1)))
    (bind _returnvalue (`|SpawnActorFromClass` (`|GetArrayItem` (`self.VehicleClass`) (`KismetMathLibrary.RandomIntegerInRange` 0 (`KismetArrayLibrary.Array_LastIndex` (`self.VehicleClass`)))) (`KismetMathLibrary.MakeTransform` (`KismetMathLibrary.MakeVector` _returnvalue_x _returnvalue_y (+ _returnvalue_z 10.0)) (`SplineComponent.GetRotationAtSplinePoint` _spline 0 "World")) "AdjustIfPossibleButDontSpawnIfColliding" "OverrideRootScale" null null))
    (`/Engine/EditorBlueprintResources/StandardMacros.IsValid` _returnvalue
      (:`Is Valid`
        (bind _asbp_base_vehicle_parent (cast `/Game/TrafficSystem/BP_BaseVehicleParent` _returnvalue)
          (:`then`
            (set `/Game/TrafficSystem/BP_BaseVehicleParent.VehicleSound?` (`self.VehicleSound?`) _asbp_base_vehicle_parent)
            (set `/Game/TrafficSystem/BP_BaseVehicleParent.DestroyIfOutRange?` (`self.DestroyIfOutRange`) _asbp_base_vehicle_parent)
            (set `/Game/TrafficSystem/BP_BaseVehicleParent.DeactiveIfOutRange?` (`self.DeactivateIfOutRange`) _asbp_base_vehicle_parent)
            (set `/Game/TrafficSystem/BP_BaseVehicleParent.DrawDebugBox` (`self.DrawDebugBox`) _asbp_base_vehicle_parent)
            (set `/Game/TrafficSystem/BP_BaseVehicleParent.PlayerMaxRange` (`self.MaxPlayerRange`) _asbp_base_vehicle_parent)
            (set `/Game/TrafficSystem/BP_BaseVehicleParent.PlayerTag` (`self.PlayerTag`) _asbp_base_vehicle_parent)
            (set `/Game/TrafficSystem/BP_BaseVehicleParent.CurrentPath` (`self.Spline`) _asbp_base_vehicle_parent)
            (set `/Game/TrafficSystem/BP_BaseVehicleParent.TimerExitParkInMin` (`self.TimeParkingInMin`) _asbp_base_vehicle_parent)
            (set `/Game/TrafficSystem/BP_BaseVehicleParent.BP_SpawnerRef` self _asbp_base_vehicle_parent)
            (`KismetArrayLibrary.Array_Add` (`self.SpawnedVehicleArray`) _asbp_base_vehicle_parent))
          (:`CastFailed`
            (`self.K2_DestroyActor` _returnvalue)))))))

(fn `CheckAndSpawnPerClass`
  (locals (RandomPointOnSpline :type Integer))
  (bind _vehicleperclass (`self.VehiclePerClass`))
  (bind _classnum (`self.ClassNum`))
  (bind _randompointonspline (`local.RandomPointOnSpline`))
  (bind _spline (`/Game/TrafficSystem/BP_SplineRoad.Spline` (`self.Spline`)))
  (bind (_returnvalue_x _returnvalue_y _returnvalue_z) (`KismetMathLibrary.BreakVector` (`SplineComponent.GetLocationAtSplinePoint` _spline _randompointonspline "World")))
  ;[1 1 1] Spawn vehicles by class and set spawner settings in vehicles
  (if (`KismetArrayLibrary.Array_IsValidIndex` _vehicleperclass _classnum)
    (set `self.TempVehicleMaxNum` (`|GetArrayItem` _vehicleperclass _classnum))
    (set `self.RandomInt` (`KismetMathLibrary.RandomIntegerInRange` 0 (`KismetArrayLibrary.Array_LastIndex` (`self.ArraySpline`))))
    (bind (_output _colliding_) (`self.CheckCollision`))
    (set `self.Spline` _output)
    (if (not _colliding_)
      (set `local.RandomPointOnSpline` (`KismetMathLibrary.RandomInteger` (- (`SplineComponent.GetNumberOfSplinePoints` _spline) 1)))
      (bind _returnvalue (`|SpawnActorFromClass` (`|GetArrayItem` (`self.VehicleClass`) (`self.ClassNum`)) (`KismetMathLibrary.MakeTransform` (`KismetMathLibrary.MakeVector` _returnvalue_x _returnvalue_y (+ _returnvalue_z 3.0)) (`SplineComponent.GetRotationAtSplinePoint` _spline _randompointonspline "World")) "AdjustIfPossibleButDontSpawnIfColliding" "OverrideRootScale" null null))
      (`/Engine/EditorBlueprintResources/StandardMacros.IsValid` _returnvalue
        (:`Is Valid`
          (bind _asbp_base_vehicle_parent (cast `/Game/TrafficSystem/BP_BaseVehicleParent` _returnvalue)
            (:`then`
              (set `/Game/TrafficSystem/BP_BaseVehicleParent.VehicleSound?` (`self.VehicleSound?`) _asbp_base_vehicle_parent)
              (set `/Game/TrafficSystem/BP_BaseVehicleParent.DestroyIfOutRange?` (`self.DestroyIfOutRange`) _asbp_base_vehicle_parent)
              (set `/Game/TrafficSystem/BP_BaseVehicleParent.DeactiveIfOutRange?` (`self.DeactivateIfOutRange`) _asbp_base_vehicle_parent)
              (set `/Game/TrafficSystem/BP_BaseVehicleParent.DrawDebugBox` (`self.DrawDebugBox`) _asbp_base_vehicle_parent)
              (set `/Game/TrafficSystem/BP_BaseVehicleParent.PlayerMaxRange` (`self.MaxPlayerRange`) _asbp_base_vehicle_parent)
              (set `/Game/TrafficSystem/BP_BaseVehicleParent.PlayerTag` (`self.PlayerTag`) _asbp_base_vehicle_parent)
              (set `/Game/TrafficSystem/BP_BaseVehicleParent.CurrentPath` (`self.Spline`) _asbp_base_vehicle_parent)
              (set `/Game/TrafficSystem/BP_BaseVehicleParent.TimerExitParkInMin` (`self.TimeParkingInMin`) _asbp_base_vehicle_parent)
              (set `/Game/TrafficSystem/BP_BaseVehicleParent.BP_SpawnerRef` self _asbp_base_vehicle_parent)
              (`KismetArrayLibrary.Array_Add` (`self.SpawnedVehicleArray`) _asbp_base_vehicle_parent)
              (bind _output_get (set `self.TempVehicleNum` (+ (`self.TempVehicleNum`) 1)))
              (if (not (< _output_get (`self.TempVehicleMaxNum`)))
                (set `self.ClassNum` (+ (`self.ClassNum`) 1))
                (set `self.TempVehicleNum` 0)))
            (:`CastFailed`
              (`self.K2_DestroyActor` _returnvalue))))))
    (else
      (`KismetSystemLibrary.K2_ClearAndInvalidateTimerHandle` (`self.TimerHandle`))
      (if (`self.RespawnDestroyedVehicle`)
        (`KismetSystemLibrary.K2_SetTimer` null "ContinueSpawn" 30.0)))))

(fn `CheckCollision`
  (returns (Output :type "/Game/TrafficSystem/BP_SplineRoad Object Reference") (`Colliding?` :type Boolean))
  (bind _output (`|GetArrayItem` (`self.ArraySpline`) (`self.RandomInt`)))
  (bind _spline (`/Game/TrafficSystem/BP_SplineRoad.Spline` _output))
  (bind _returnvalue (`SceneComponent.GetForwardVector` _spline))
  (bind _returnvalue_2 (`SceneComponent.K2_GetComponentLocation` _spline))
  ;[1 1 1] Check if there are any vehicles on the spawn points
  (bind (_outhit _returnvalue_3) (`KismetSystemLibrary.BoxTraceSingleForObjects` (+ (+ (* _returnvalue 350.0) (0.0 0.0 80.0)) _returnvalue_2) (+ (+ (* _returnvalue -350.0) (0.0 0.0 80.0)) _returnvalue_2) (0.0 80.0 2.0) (`SceneComponent.K2_GetComponentRotation` _spline) (`|MakeArray` "ObjectTypeQuery2" "ObjectTypeQuery3" "ObjectTypeQuery5" :!type "EObjectTypeQuery Enum")))
  (return _output _returnvalue_3))

(fn `ContinueSpawn`
  ;[1 1 1] If "Respawn Destroyed Vehicle" is true, check the number of vehicles is less than the set limit and if true, continue spawning
  (if (`self.RespawnDestroyedVehicle`)
    (if (< (`KismetArrayLibrary.Array_Length` (`self.SpawnedVehicleArray`)) (`self.MaxVehicle`))
      (bind _returnvalue (`KismetSystemLibrary.K2_SetTimer` null "GoToRandomSpawn" 1.0 true))
      (set `self.TimerHandle` _returnvalue)
      (else
        (bind _returnvalue_2 (`KismetSystemLibrary.K2_SetTimer` null "ContinueSpawn" 30.0))
        (set `self.TimerHandle` _returnvalue_2)))
    (else
      (`KismetSystemLibrary.K2_ClearAndInvalidateTimerHandle` (`self.TimerHandle`)))))

(fn `GoToRandomSpawn`
  (`self.SpawnRandom`))

(fn `UserConstructionScript`)