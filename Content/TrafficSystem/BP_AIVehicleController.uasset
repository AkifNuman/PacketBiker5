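; AI controller that drives a traffic vehicle along road splines, either wandering or heading to a destination.
; A looping 0.1-second timer, instead of Tick, runs a spawner-dependent collision check, then spline driving, then applies throttle, brake and steering.
; Steering chases a look-ahead spline point, which also triggers next-path selection; throttle follows speed limits and spline position.
; Overrides handle vehicles ahead, stop systems, priority, highway entry and reversing when stuck.
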(event `DisableDriveTick`
  ;[1 1 1] disable drive timer loop
  (`KismetSystemLibrary.K2_ClearAndInvalidateTimerHandle` (`self.TimerHandle`)))

(event `EnableDriveTick`
  ;[1 1 1] enable drive tick loop
  (`KismetSystemLibrary.K2_ClearAndInvalidateTimerHandle` (`self.TimerHandle`))
  (bind _returnvalue (`KismetSystemLibrary.K2_SetTimer` null "DriveTick" 0.1 true))
  (set `self.TimerHandle` _returnvalue))

(event `self.ReceiveBeginPlay`
  (`KismetSystemLibrary.K2_SetTimer` null "RestartDrive" 0.5))

(event `RestartDrive`
  (`self.ControlledCar`
    (:`then`
      _)
    (:`else`
      (bind _asbp_base_vehicle_parent (cast `/Game/TrafficSystem/BP_BaseVehicleParent` (`self.K2_GetPawn`)))
      (set `self.ControlledCar` _asbp_base_vehicle_parent)))
  (`self.Set Spline` (`/Game/TrafficSystem/BP_BaseVehicleParent.CurrentPath` (`self.ControlledCar`)))
  (`self.ChooseFunction`)
  (`self.EnableDriveTick`))

(event `DriveTick`
  (bind _controlledcar (`self.ControlledCar`))
  ;[1 1 1] Drive Tick
  (`self.ControlledCar`
    (:`then`
      (if (not (`self.ArrivedAtDestination?`))
        (if (not (`/Game/TrafficSystem/BP_BaseVehicleParent.Destination?` _controlledcar))
          (`self.CurrentPath` :!label _label
            (:`then`
              (`self.CollisionSwitch`)
              (`self.SplineDrive`))
            (:`else`
              (set `self.Throttle` 0.0)
              (set `self.SteeringToApply` 0.0)))
          (`self.ApplyThrottleAndSteering`)
          (elif (> (`KismetMathLibrary.VSize` (- (`self.K2_GetActorLocation` _controlledcar) (`/Game/TrafficSystem/BP_BaseVehicleParent.DestinationLocation` _controlledcar))) 150.0)
            (goto _label)
            (else
              (set `self.ArrivedAtDestination?` true)
              (`self.DisableDriveTick`))))
        (else
          ;[1 1 1] if destination is reached, stop vehicle
          (set `self.Throttle` (select `bool` (>= (`self.SpeedtoKMh`) 0.2) :`true` -1.0))
          (set `self.SteeringToApply` 0.0))))
    (:`else`
      (goto _label))))

(event `ExitParking`
  (`self.ApplyThrottleAndSteering`))

(event `DelayCheck`
  ;[1 1 1] Check if vehicle is still stuck
  (`KismetSystemLibrary.K2_SetTimer` null "DelayCheckFunc" 5.0))

(event `ReverseEvent`
  (params (Steering :type "Float (double-precision)"))
  ;[1 1 1] reverse
  (set `self.Reverse` true)
  (set `self.SteeringToApply` Steering)
  (`KismetSystemLibrary.K2_SetTimer` null "DisableReverse" 1.5))

(event `SelectNewSpline`
  (bind _controlledcar (`self.ControlledCar`))
  (bind _currentpath (`self.CurrentPath`))
  (bind _controlledcar_2 (`self.ControlledCar`))
  (bind _currentpath_2 (`self.CurrentPath`))
  ;[1 1 1] Check and select new spline
  (`/Engine/EditorBlueprintResources/StandardMacros.DoOnce` false :!label _label_2
    (:`Completed`
      (set `/Game/TrafficSystem/BP_BaseVehicleParent.OldPath` (`/Game/TrafficSystem/BP_BaseVehicleParent.CurrentPath` _controlledcar_2) _controlledcar_2)
      (if (`/Game/TrafficSystem/BP_BaseVehicleParent.Destination?` _controlledcar_2)
        (bind (_validspline _direction) (`/Game/TrafficSystem/BP_SplineRoad.MoveToDestination` _currentpath_2 (`/Game/TrafficSystem/BP_BaseVehicleParent.DestinationLocation` (`self.ControlledCar`))))
        (set `/Game/TrafficSystem/BP_BaseVehicleParent.NextSpline` _validspline _controlledcar)
        (set `/Game/TrafficSystem/BP_BaseVehicleParent.NextDirection` _direction _controlledcar)
        (else
          (bind (_validspline_2 _nextdirection) (`/Game/TrafficSystem/BP_SplineRoad.SetNewSpline` _currentpath_2))
          (set `/Game/TrafficSystem/BP_BaseVehicleParent.NextSpline` _validspline_2 _controlledcar)
          (set `/Game/TrafficSystem/BP_BaseVehicleParent.NextDirection` _nextdirection _controlledcar)))
      (if (`/Game/TrafficSystem/BP_SplineRoad.StopSystem` _currentpath)
        (`/Game/TrafficSystem/BP_SplineRoad.StopSystemSplineCheck` _currentpath (`/Game/TrafficSystem/BP_BaseVehicleParent.NextDirection` _controlledcar))))))

(event `ResetDoOnce`
  ;[1 1 1] Check and select new spline
  (goto _label_2 :!via `Reset`))

(fn `ApplyThrottleAndSteering`
  (bind _throttle (`self.Throttle`))
  (bind _controlledcar (`self.ControlledCar`))
  (bind _controlledcar_2 (`self.ControlledCar`))
  (bind _returnvalue (* (`self.Throttle`) -1.0))
  (bind _returnvalue_2 (<= _throttle 0.0))
  (bind _vehiclemovementcomponent (`WheeledVehiclePawn.VehicleMovementComponent` (`self.ControlledCar`)))
  ;[1 1 1] Apply throttle and steering to vehicle
  (`ChaosVehicleMovementComponent.SetSteeringInput` _vehiclemovementcomponent (`self.SteeringToApply`))
  (if (> _throttle 0.0)
    (`ChaosVehicleMovementComponent.SetThrottleInput` _vehiclemovementcomponent (`self.Throttle`))
    (`ChaosVehicleMovementComponent.SetBrakeInput` _vehiclemovementcomponent 0.0)
    (if (`/Game/TrafficSystem/BP_BaseVehicleParent.Handbreak` _controlledcar) :!label _label
      (set `/Game/TrafficSystem/BP_BaseVehicleParent.Handbreak` false _controlledcar))
    (else
      (`ChaosVehicleMovementComponent.SetThrottleInput` _vehiclemovementcomponent 0.0)
      (`ChaosVehicleMovementComponent.SetBrakeInput` _vehiclemovementcomponent (select `bool` (`self.Reverse`) :`false` (select `bool` _returnvalue_2 :`false` _returnvalue :`true` 1.0) :`true` _returnvalue))
      (if _returnvalue_2
        (if (`self.ParkEnabled`)
          (goto _label)
          (elif (not (`/Game/TrafficSystem/BP_BaseVehicleParent.Handbreak` _controlledcar_2))
            (set `/Game/TrafficSystem/BP_BaseVehicleParent.Handbreak` true _controlledcar_2)))
        (else
          (goto _label))))))

(fn `CalculateThrottle`
  (returns (Throttle :type "Float (double-precision)"))
  (locals (SpeedLocal :type "Float (double-precision)" :default 0.0) (VelocitySplineLengthLocal :type "Float (double-precision)" :default 0.0))
  (bind _speedlocal (`local.SpeedLocal`))
  (bind _velocitysplinelengthlocal (`local.VelocitySplineLengthLocal`))
  (bind _splinelength (`self.SplineLength`))
  (bind _maxspeedonspline (`/Game/TrafficSystem/BP_SplineRoad.MaxSpeedOnSpline` (`self.CurrentPath`)))
  (bind _stopsystem (`/Game/TrafficSystem/BP_SplineRoad.StopSystem` (`self.CurrentPath`)))
  (bind _returnvalue (/ (* _splinelength 60.0) 100.0))
  (set `local.SpeedLocal` (`self.SpeedtoKMh`))
  (if (`/Game/TrafficSystem/BP_SplineRoad.HighSpeedRoad` (`self.CurrentPath`))
    ;[1 1 1] Throttle on highway
    (if (> (`local.SpeedLocal`) (`/Game/TrafficSystem/BP_SplineRoad.MaxSpeedOnSpline` (`self.CurrentPath`)))
      (return 0.1)
      (else
        (return 0.8)))
    (else
      (if (< (`self.CarDistanceToSpline`) 450.0)
        (if (< (`local.SpeedLocal`) 15.0)
          _
          (else
            (return (`KismetMathLibrary.MapRangeClamped` (`local.SpeedLocal`) 40.0 5.0 -1.0)))))
      (if (< (`local.SpeedLocal`) 1.0)
        (return 0.5)
        (elif (< (`local.SpeedLocal`) _maxspeedonspline)
          (bind _output_get (set `local.VelocitySplineLengthLocal` (`self.VelocityBySplineLength`)))
          (if (== _output_get 0.0)
            (return 0.5)
            (else
              (return (select `bool` (< _velocitysplinelengthlocal _returnvalue) :`false` (`KismetMathLibrary.MapRangeClamped` _velocitysplinelengthlocal _returnvalue _splinelength 0.5 (select `bool` _stopsystem :`false` (select `bool` (>= _speedlocal 20.0) :`false` 0.3 :`true` 0.15) :`true` (select `bool` (>= _speedlocal 10.0) :`false` 0.3 :`true` 0.15))) :`true` (select `bool` _stopsystem :`false` (`KismetMathLibrary.MapRangeClamped` _velocitysplinelengthlocal 0.0 _returnvalue 0.9 0.3) :`true` (`KismetMathLibrary.MapRangeClamped` _velocitysplinelengthlocal 0.0 _returnvalue 0.9 0.3))))))
          (else
            ;[1 1 1] Slow down if the speed is above the limit
            (return (`KismetMathLibrary.MapRangeClamped` (`local.SpeedLocal`) 120.0 _maxspeedonspline -0.6 0.1))))))))

(fn `CheckDistancetoLastPoint`
  (params (SplineToCheck :type "/Game/TrafficSystem/BP_SplineRoad Object Reference"))
  (bind _spline (`/Game/TrafficSystem/BP_SplineRoad.Spline` SplineToCheck))
  (if (<= (`KismetMathLibrary.VSize` (- (`SplineComponent.GetLocationAtSplinePoint` _spline (- (`SplineComponent.GetNumberOfSplinePoints` _spline) 1) "World") (`self.K2_GetActorLocation` (`self.ControlledCar`)))) 800.0)
    (bind _returnhit (`/Game/TrafficSystem/BP_SplineRoad.StopSystemVehicleCheck` (`local.SplineToCheck`) (`self.ControlledCar`)))
    (if _returnhit
      (set `self.Hit?` true)))
  (return))

(fn `ChooseFunction`
  (bind _controlledcar (`self.ControlledCar`))
  ;[1 1 1] Choose according to the spawner settings
  (if (`/Game/TrafficSystem/BP_BaseVehicleParent.DeactiveIfOutRange?` _controlledcar)
    (set `self.TickSelected` 1)
    (elif (`/Game/TrafficSystem/BP_BaseVehicleParent.DestroyIfOutRange?` _controlledcar)
      (set `self.TickSelected` 2)
      (else
        (set `self.TickSelected` 3)))))

(fn `CollisionSwitch`
  (bind _controlledcar (`self.ControlledCar`))
  (switch `int` (`self.TickSelected`)
    (:`1`
      (`/Game/TrafficSystem/BP_BaseVehicleParent.CollisionTickWithDeactivation` _controlledcar))
    (:`2`
      (`/Game/TrafficSystem/BP_BaseVehicleParent.CollisionTickWithDestroy` _controlledcar))
    (:`3`
      (`/Game/TrafficSystem/BP_BaseVehicleParent.CollisionTick` _controlledcar))))

(fn `DelayCheckFunc`
  (if (< (`self.SpeedtoKMh`) 0.1)
    (set `self.HitAndGo` false)
    (set `self.Reverse` true)
    (`KismetSystemLibrary.K2_SetTimer` null "DisableReverse" 1.5)))

(fn `DisableReverse`
  (set `self.Reverse` false)
  (`self.EnableDriveTick`))

(fn `GetRotationXVector`
  (params (Start :type "Vector Structure"))
  (returns (`Return Value Z (Yaw)` :type "Float (single-precision)"))
  (bind (_returnvalue_roll _returnvalue_pitch _returnvalue_yaw) (`KismetMathLibrary.BreakRotator` (`KismetMathLibrary.Conv_VectorToRotator` (`KismetMathLibrary.InverseTransformDirection` (`self.GetTransform` (`self.ControlledCar`)) (`KismetMathLibrary.Conv_RotatorToVector` (`KismetMathLibrary.FindLookAtRotation` Start (`self.SplinePosition`)))))))
  ;[1 1 1] Get Z Rotation from x Vector
  (return _returnvalue_yaw))

(fn `GetSplinePosition`
  (returns (ClosestLocation :type "Vector Structure"))
  (locals (LocClosestLocation :type "Vector Structure"))
  (bind _controlledcar (`self.ControlledCar`))
  (bind _returnvalue (`self.K2_GetActorLocation` (`self.ControlledCar`)))
  (bind _oldpath (`/Game/TrafficSystem/BP_BaseVehicleParent.OldPath` (`self.ControlledCar`)))
  (bind _spline (`/Game/TrafficSystem/BP_SplineRoad.Spline` (`self.CurrentPath`)))
  (set `local.LocClosestLocation` (`SplineComponent.FindLocationClosestToWorldLocation` _spline (+ (* (`KismetMathLibrary.Normal` (`SplineComponent.FindTangentClosestToWorldLocation` _spline _returnvalue "World")) (select `bool` (`/Game/TrafficSystem/BP_SplineRoad.HighSpeedRoad` (`self.CurrentPath`)) :`false` (`self.SplineLookDistance`) :`true` 1500.0 :!type "Float (single-precision)")) _returnvalue) "World"))
  (bind _output_get (set `self.CarDistanceToSpline` (`KismetMathLibrary.VSize` (- (`local.LocClosestLocation`) _returnvalue))))
  (if (> _output_get 300.0)
    (if (>= (`self.CarDistanceToSpline`) 800.0)
      (`/Game/TrafficSystem/BP_BaseVehicleParent.PriorityEvent` (`self.ControlledCar`))
      (else
        (`self.SelectNewSpline`)
        (set `/Game/TrafficSystem/BP_BaseVehicleParent.Priority` false (`self.ControlledCar`))))
    (else
      (bind _output_get_2 (set `/Game/TrafficSystem/BP_BaseVehicleParent.CurrentPath` (`/Game/TrafficSystem/BP_BaseVehicleParent.NextSpline` _controlledcar) _controlledcar))
      (`self.Set Spline` _output_get_2)
      (`self.ResetDoOnce`)
      (if (not (`/Game/TrafficSystem/BP_BaseVehicleParent.Destination?` (`self.ControlledCar`)))
        (`/Game/TrafficSystem/BP_BaseVehicleParent.ResetParkingCheck` (`self.ControlledCar`)))))
  (if (`/Game/TrafficSystem/BP_SplineRoad.StopSystem` _oldpath)
    (`self.CheckDistancetoLastPoint` _oldpath))
  (return (`local.LocClosestLocation`)))

(fn `HighwayEnterCollisionCheck`
  (params (SplineRoad :type "/Game/TrafficSystem/BP_SplineRoad Object Reference"))
  (bind _spline (`/Game/TrafficSystem/BP_SplineRoad.Spline` SplineRoad))
  (bind _returnvalue (`SceneComponent.GetForwardVector` _spline))
  (bind _returnvalue_2 (+ (`SplineComponent.FindLocationClosestToWorldLocation` _spline (`self.K2_GetActorLocation` (`self.ControlledCar`)) "World") (0.0 0.0 40.0)))
  (bind (_outhit _returnvalue_3) (`KismetSystemLibrary.LineTraceSingleForObjects` :`Start` (+ (* _returnvalue -4000.0) _returnvalue_2) :`End` (+ (* _returnvalue 1500.0) _returnvalue_2) :`ObjectTypes` (`|MakeArray` "ObjectTypeQuery5" :!type "EObjectTypeQuery Enum") :`DrawDebugType` "ForDuration" :`DrawTime` 0.1))
  (if _returnvalue_3
    (set `self.CanEnterHighway` false)
    (else
      (set `self.CanEnterHighway` true))))

(fn `ReverseMode`
  (set `self.SteeringToApply` (* (`self.SteeringToApply`) 1.7))
  (set `self.Throttle` (* -1 (`KismetMathLibrary.MapRangeClamped` (`KismetMathLibrary.Abs` (`self.GetRotationXVector` (`self.K2_GetActorLocation` (`self.ControlledCar`)))) 0.0 35.0 0.4 0.2))))

(fn `Set Spline`
  (params (Path :type "/Game/TrafficSystem/BP_SplineRoad Object Reference"))
  (bind _currentpath (`self.CurrentPath`))
  ;[1 1 1] Set new spline and spline length
  (`/Engine/EditorBlueprintResources/StandardMacros.IsValid` Path
    (:`Is Valid`
      (set `self.CurrentPath` Path))
    (:`Is Not Valid`
      (`/Engine/EditorBlueprintResources/StandardMacros.IsValid` _currentpath
        (:`Is Valid`
          _))))
  (set `self.SplineLength` (`SplineComponent.GetSplineLength` (`/Game/TrafficSystem/BP_SplineRoad.Spline` _currentpath))))

(fn `SetNewPath`
  (params (NewPath :type "/Game/TrafficSystem/BP_SplineRoad Object Reference"))
  (`/Engine/EditorBlueprintResources/StandardMacros.IsValid` NewPath
    (:`Is Valid`
      (`self.Set Spline` NewPath))
    (:`Is Not Valid`
      (set `self.CurrentPath` null))))

(fn `SpeedtoKMh`
  (returns (ReturnValue :type "Float (double-precision)"))
  (return (* (`ChaosVehicleMovementComponent.GetForwardSpeed` (`WheeledVehiclePawn.VehicleMovementComponent` (`self.ControlledCar`))) 0.036)))

(fn `SplineDrive`
  (bind _throttle (`self.Throttle`))
  (bind _controlledcar (`self.ControlledCar`))
  (bind _controlledcar_2 (`self.ControlledCar`))
  (bind _returnvalue (`self.K2_GetActorLocation` _controlledcar))
  (set `self.SplinePosition` (`self.GetSplinePosition`))
  (if (not (`self.HitAndGo`))
    (if (`self.Reverse`)
      ;[1 1 1] Reverse mode
      (`self.ReverseMode`)
      (elif (not (or (`self.Hit?`) (not (`self.CanEnterHighway`))))
        (if (not (`self.CarInFront`))
          ;[1 1 1] Normale Drive
          (bind _throttle_2 (`self.CalculateThrottle`))
          (bind _throttlemultiplier (`self.SteeringAndThrottleMultiplier`))
          (set `self.Throttle` (* _throttlemultiplier (`KismetMathLibrary.FClamp` _throttle_2 -1.0)))
          (else
            ;[1 1 1] if vehicle hit another but is distant, decelerates
            (bind _throttlemultiplier_2 (`self.SteeringAndThrottleMultiplier`))
            (if (> (`self.SpeedtoKMh`) (`/Game/TrafficSystem/BP_BaseVehicleParent.FrontCarSpeed` (`self.ControlledCar`)))
              (set `self.Throttle` (`KismetMathLibrary.FClamp` (- (* _throttlemultiplier_2 (`self.Throttle`)) 0.2))))))
        (elif (`/Game/TrafficSystem/BP_BaseVehicleParent.Priority` (`self.ControlledCar`))
          ;[1 1 1] if vehicle have priority
          (set `self.Throttle` (select `bool` (> (`self.SpeedtoKMh`) 1.0) :`true` -1.0))
          (else
            ;[1 1 1] if hit another vehicle
            (set `self.Throttle` (`KismetMathLibrary.MapRangeClamped` (`KismetMathLibrary.VSize` (- (`SceneComponent.K2_GetComponentLocation` (`WheeledVehiclePawn.Mesh` _controlledcar_2)) (`self.ImpactPoint`))) (`/Game/TrafficSystem/BP_BaseVehicleParent.DistanceTrace` _controlledcar_2) 350.0 (select `bool` (< (`self.SpeedtoKMh`) 1.0) :`false` -1.0) (select `bool` (> _throttle 0.0) :`true` (- _throttle 0.2))))))))
    (else
      ;[1 1 1] if vehicle hit another front box component
      (set `self.SteeringToApply` (* (`KismetMathLibrary.Dot_VectorVector` (`KismetMathLibrary.Normal` (`KismetMathLibrary.GetDirectionUnitVector` _returnvalue (`self.ImpactPoint`))) (`KismetMathLibrary.Normal` (`KismetMathLibrary.GetRightVector` (`self.K2_GetActorRotation` _controlledcar)))) -1.5))
      (set `self.Throttle` (`KismetMathLibrary.MapRangeClamped` (`KismetMathLibrary.Abs` (`self.GetRotationXVector` _returnvalue)) 0.0 35.0 0.4 0.2))
      (`self.DelayCheck`))))

(fn `SteeringAndThrottleMultiplier`
  (returns (ThrottleMultiplier :type "Float (double-precision)"))
  (bind _returnvalue (`self.SpeedtoKMh`))
  (bind _maxspeedonspline (`/Game/TrafficSystem/BP_SplineRoad.MaxSpeedOnSpline` (`self.CurrentPath`)))
  (bind _return_value_z__yaw_ (`self.GetRotationXVector` (`self.K2_GetActorLocation` (`self.ControlledCar`))))
  (bind _returnvalue_2 (select `bool` (< (`self.CarDistanceToSpline`) 600.0) :`false` (`KismetMathLibrary.MapRangeClamped` _return_value_z__yaw_ -180.0 180.0 -3.5 3.5) :`true` (`KismetMathLibrary.MapRangeClamped` _return_value_z__yaw_ -180.0 180.0 -5.0 5.0)))
  (set `self.SteeringToApply` (select `bool` (`/Game/TrafficSystem/BP_BaseVehicleParent.HitAround?` (`self.ControlledCar`)) :`false` _returnvalue_2 :`true` (`self.SteeringOnHit`)))
  (return (* -1 (select `bool` (`/Game/TrafficSystem/BP_SplineRoad.HighSpeedRoad` (`self.CurrentPath`)) :`false` (`KismetMathLibrary.MapRangeClamped` (`KismetMathLibrary.Abs` _returnvalue_2) 0.0 5.0 -1.0 -0.1) :`true` (select `bool` (> _returnvalue _maxspeedonspline) :`false` (`KismetMathLibrary.MapRangeClamped` _returnvalue 0.0 _maxspeedonspline -1.0 -0.8) :`true` (`KismetMathLibrary.MapRangeClamped` (`KismetMathLibrary.Abs` _return_value_z__yaw_) 0.0 7.0 -1.0 -0.1))))))

(fn `UserConstructionScript`)

(fn `VelocityBySplineLength`
  (returns (VectorLength :type "Float (double-precision)"))
  ;[1 1 1] Calculate the distance on spline and adjust speed (on function CalculateThrottle)
  (bind _currentpath (`self.CurrentPath`)
    (:`then`
      (return (`KismetMathLibrary.VSize` (- (`SplineComponent.GetLocationAtSplinePoint` (`/Game/TrafficSystem/BP_SplineRoad.Spline` _currentpath) 0 "World") (`self.SplinePosition`)))))
    (:`else`
      (return 50.0))))