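; BP_SplineRoad is a traffic-system road segment linked to straight, right and left successors; on BeginPlay it snaps parking splines' first points onto itself.
; It picks a vehicle's next segment at random among trace-detected empty branches, else the least busy, or nearest a destination; high-speed roads continue straight.
; At junctions, it selects priority splines by drive side and turn, then line-traces them for vehicles, considering speed, stop signs and traffic lights to report conflicts.
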(event `self.ReceiveBeginPlay`
  ;[1 1 1] Check if there are parking spaces on this spline and if it finds them, move Spline Point 0 on the street line
  (for _array_element (`self.ParkingOnThisSpline`)
    (bind _parkspline (`/Game/TrafficSystem/BP_ParkingSpot.ParkSpline` _array_element))
    (`SplineComponent.SetLocationAtSplinePoint` _parkspline 0 (`SplineComponent.FindLocationClosestToWorldLocation` (`self.Spline`) (`SplineComponent.GetLocationAtSplinePoint` _parkspline 0 "World") "World") "World" true)))

(fn `LineTraceToCheckSpline`
  (params (Spline :type "/Game/TrafficSystem/BP_SplineRoad Object Reference"))
  (returns (OutHits :type "Array of HitResult Structure"))
  (bind _spline (`/Game/TrafficSystem/BP_SplineRoad.Spline` Spline))
  (bind _returnvalue (`SplineComponent.GetLocationAtSplinePoint` _spline 1 "World"))
  (bind _returnvalue_2 (`SplineComponent.GetLocationAtSplinePoint` _spline 0 "World"))
  (bind _returnvalue_3 (`KismetMathLibrary.GetForwardVector` (`SceneComponent.K2_GetComponentRotation` (`/Game/TrafficSystem/BP_SplineRoad.Arrow` Spline))))
  (bind _returnvalue_4 (+ _returnvalue_2 (0.0 0.0 40.0)))
  (bind _outhits (`KismetSystemLibrary.LineTraceMultiForObjects` (+ (* _returnvalue_3 -350.0) _returnvalue_4) (select `bool` (< (`KismetMathLibrary.VSize` (- _returnvalue_2 _returnvalue)) 2000.0) :`false` (+ (* _returnvalue_3 2000.0) _returnvalue_4) :`true` (+ _returnvalue (0.0 0.0 40.0))) (`|MakeArray` "ObjectTypeQuery5" :!type "EObjectTypeQuery Enum")))
  (return _outhits))

(fn `MoveToDestination`
  (params (Location :type "Vector Structure"))
  (returns (ValidSpline :type "/Game/TrafficSystem/BP_SplineRoad Object Reference") (Direction :type String))
  (bind _indexofminvalue (`KismetMathLibrary.MinOfFloatArray` (`self.DistanceToDestinatio`)))
  (`KismetArrayLibrary.Array_Clear` (`self.DistanceToDestinatio`))
  (`KismetArrayLibrary.Array_Clear` (`self.ValidSpline`))
  (`KismetArrayLibrary.Array_Clear` (`self.Directions`))
  (bind _straightspline (`self.StraightSpline`)
    (:`then`
      (`KismetArrayLibrary.Array_AddUnique` (`self.ValidSpline`) _straightspline)
      (`KismetArrayLibrary.Array_AddUnique` (`self.Directions`) "Straight"))
    (:`else`
      _))
  (bind _rightspline (`self.RightSpline`)
    (:`then`
      (`KismetArrayLibrary.Array_AddUnique` (`self.ValidSpline`) _rightspline)
      (`KismetArrayLibrary.Array_AddUnique` (`self.Directions`) "Right"))
    (:`else`
      _))
  (bind _leftspline (`self.LeftSpline`)
    (:`then`
      (`KismetArrayLibrary.Array_AddUnique` (`self.ValidSpline`) _leftspline)
      (`KismetArrayLibrary.Array_AddUnique` (`self.Directions`) "Left"))
    (:`else`
      _))
  (for _array_element (`self.ValidSpline`)
    (`KismetArrayLibrary.Array_AddUnique` (`self.DistanceToDestinatio`) (`KismetMathLibrary.VSize` (- (`self.K2_GetActorLocation` _array_element) (`local.Location`)))))
  (return (`|GetArrayItem` (`self.ValidSpline`) _indexofminvalue) (`|GetArrayItem` (`self.Directions`) _indexofminvalue)))

(fn `SetNewSpline`
  (returns (ValidSpline :type "/Game/TrafficSystem/BP_SplineRoad Object Reference") (NextDirection :type String))
  (bind _path (`self.Path`))
  (bind _validspline (`self.ValidSpline`))
  (bind _indexofminvalue (`KismetMathLibrary.MinOfIntArray` (`self.VehicleOnSpline`)))
  (bind _output (`|GetArrayItem` _path (`KismetMathLibrary.RandomIntegerInRange` 0 (`KismetArrayLibrary.Array_LastIndex` _path))))
  (if (not (`self.HighSpeedRoad`))
    (`KismetArrayLibrary.Array_Clear` (`self.Path`))
    (`KismetArrayLibrary.Array_Clear` (`self.ValidSpline`))
    (`KismetArrayLibrary.Array_Clear` (`self.VehicleOnSpline`))
    (`KismetArrayLibrary.Array_Clear` (`self.Directions`))
    (bind _straightspline (`self.StraightSpline`)
      (:`then`
        (`KismetArrayLibrary.Array_AddUnique` (`self.ValidSpline`) _straightspline)
        (`KismetArrayLibrary.Array_AddUnique` (`self.Directions`) "Straight"))
      (:`else`
        _))
    (bind _rightspline (`self.RightSpline`)
      (:`then`
        (`KismetArrayLibrary.Array_AddUnique` (`self.ValidSpline`) _rightspline)
        (`KismetArrayLibrary.Array_AddUnique` (`self.Directions`) "Right"))
      (:`else`
        _))
    (bind _leftspline (`self.LeftSpline`)
      (:`then`
        (`KismetArrayLibrary.Array_AddUnique` (`self.ValidSpline`) _leftspline)
        (`KismetArrayLibrary.Array_AddUnique` (`self.Directions`) "Left"))
      (:`else`
        _))
    (if (> (`KismetArrayLibrary.Array_Length` (`self.ValidSpline`)) 1)
      (for _array_element (`self.ValidSpline`)
        ;[1 1 1] Check the number of vehicles on the spline, so as not to create traffic
        (bind _outhits (`self.LineTraceToCheckSpline` _array_element))
        (`KismetArrayLibrary.Array_AddUnique` (`self.VehicleOnSpline`) (`KismetArrayLibrary.Array_Length` _outhits)))
      ;[1 1 1] Check the number of vehicles on the spline is less than 1 and add them to "Path" if true
      (for (_array_element_2 _array_index) (`self.VehicleOnSpline`)
        (if (< _array_element_2 1)
          (`KismetArrayLibrary.Array_AddUnique` (`self.Path`) _array_index)))
      ;[1 1 1] If "Path" (array) has at least one value, it returns a random street among those available
      (if (`KismetArrayLibrary.Array_IsValidIndex` (`self.Path`))
        (return (`|GetArrayItem` (`self.ValidSpline`) _output) (`|GetArrayItem` (`self.Directions`) _output))
        (elif (`KismetArrayLibrary.Array_IsValidIndex` _validspline)
          (return (`|GetArrayItem` _validspline _indexofminvalue) (`|GetArrayItem` (`self.Directions`) _indexofminvalue))
          (else
            (return null ""))))
      (else
        (return (`|GetArrayItem` (`self.ValidSpline`)) (`|GetArrayItem` (`self.Directions`)))))
    (else
      (return (`self.StraightSpline`) "Straight"))))

(fn `StopSystemSplineCheck`
  (params (VehicleDirection :type String))
  (set `self.Direction` VehicleDirection)
  (`BlueprintMapLibrary.Map_Clear` (`self.SplineStopCheck`))
  (switch `string` (`self.DriveLane`)
    (:`Right`
      (switch `string` (`self.Direction`)
        (:`Straight`
          (bind _piorityright (`self.PiorityRight`)
            (:`then`
              (`BlueprintMapLibrary.Map_Add` (`self.SplineStopCheck`) 2 _piorityright))
            (:`else`
              _)))
        (:`Right`
          _)
        (:`Left`
          (bind _pioritystraight (`self.PiorityStraight`)
            (:`then`
              (`BlueprintMapLibrary.Map_Add` (`self.SplineStopCheck`) 0 _pioritystraight))
            (:`else`
              _))
          (bind _piorityright_2 (`self.PiorityRight`)
            (:`then`
              (`BlueprintMapLibrary.Map_Add` (`self.SplineStopCheck`) 2 _piorityright_2))
            (:`else`
              _)))))
    (:`Left`
      (switch `string` (`self.Direction`)
        (:`Straight`
          (bind _piorityleft (`self.PiorityLeft`)
            (:`then`
              (`BlueprintMapLibrary.Map_Add` (`self.SplineStopCheck`) 1 _piorityleft))
            (:`else`
              _)))
        (:`Right`
          (bind _piorityleft_2 (`self.PiorityLeft`)
            (:`then`
              (`BlueprintMapLibrary.Map_Add` (`self.SplineStopCheck`) 1 _piorityleft_2))
            (:`else`
              _))
          (bind _pioritystraight_2 (`self.PiorityStraight`)
            (:`then`
              (`BlueprintMapLibrary.Map_Add` (`self.SplineStopCheck`) 0 _pioritystraight_2))
            (:`else`
              _)))
        (:`Left`
          _))))
  (return))

(fn `StopSystemVehicleCheck`
  (params (Vehicle :type "/Game/TrafficSystem/BP_BaseVehicleParent Object Reference"))
  (returns (ReturnHit :type Boolean))
  (locals (LocIntDirection :type Integer) (LocHit :type Boolean :default false) (VehicleOnSplineCheck :type "/Game/TrafficSystem/BP_BaseVehicleParent Object Reference"))
  (bind _splinestopcheck (`self.SplineStopCheck`))
  (bind _returnvalue (<= (`/Game/TrafficSystem/BP_BaseVehicleParent.SpeedToKMH` (`local.VehicleOnSplineCheck`)) 1.0))
  (bind _spline (`/Game/TrafficSystem/BP_SplineRoad.Spline` (`BlueprintMapLibrary.Map_Find` _splinestopcheck (`local.LocIntDirection`))))
  (bind _returnvalue_2 (`SceneComponent.GetForwardVector` _spline))
  (bind _returnvalue_3 (+ (`SplineComponent.GetLocationAtSplinePoint` _spline (- (`SplineComponent.GetNumberOfSplinePoints` _spline) 1) "World") (0.0 0.0 40.0)))
  (bind _keys (`BlueprintMapLibrary.Map_Keys` _splinestopcheck))
  (for _array_element _keys
    (set `local.LocIntDirection` _array_element)
    (bind (_outhit _returnvalue_4) (`KismetSystemLibrary.LineTraceSingleForObjects` (+ (* _returnvalue_2 -450.0) _returnvalue_3) (+ (* _returnvalue_2 (select `bool` (== (`local.LocIntDirection`) 0) :`false` 550.0 :`true` 800.0 :!type "Float (single-precision)")) _returnvalue_3) (`|MakeArray` "ObjectTypeQuery5" :!type "EObjectTypeQuery Enum") false (`|MakeArray` (`local.Vehicle`) :!type "Actor Object Reference") "None" false))
    (if _returnvalue_4
      (bind _output_get (set `local.VehicleOnSplineCheck` (cast `/Game/TrafficSystem/BP_BaseVehicleParent` (`.HitActor` (`GameplayStatics.BreakHitResult` _outhit)) :!pure true)))
      (bind _oldpath (`/Game/TrafficSystem/BP_BaseVehicleParent.OldPath` _output_get))
      (if (`/Game/TrafficSystem/BP_SplineRoad.StopSystem` _oldpath)
        (if (and (!= (`self.Direction`) "Right") (not _returnvalue))
          (set `local.LocHit` true))
        (elif (`KismetSystemLibrary.IsValid` (`/Game/TrafficSystem/BP_SplineRoad.Ref_TrafficLight` _oldpath))
          (if (not _returnvalue)
            (set `local.LocHit` true :!label _label))
          (else
            (goto _label))))))
  (return (`local.LocHit`)))

(fn `UserConstructionScript`)