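; Highway entry trigger for AI traffic that has a vehicle check for collisions against the next road while inside it.
; On the server, a DoOnce-gated begin overlap stores the vehicle and loops a short timer calling its AI controller's HighwayEnterCollisionCheck.
; Any end overlap resets the gate, sets CanEnterHighway on the stored vehicle's controller and clears the timer.
; An inline spline-based line trace remains unconnected.
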(event `CheckVehicle`
  (`/Game/TrafficSystem/BP_AIVehicleController.HighwayEnterCollisionCheck` (`/Game/TrafficSystem/BP_BaseVehicleParent.Ref_AiController` (`self.Ref_Vehicle`)) (`self.NextRoad`)))

(event `self.CollisionComponent.OnComponentBeginOverlap`
  (params (OverlappedComponent :type "PrimitiveComponent Object Reference") (OtherActor :type "Actor Object Reference") (OtherComp :type "PrimitiveComponent Object Reference") (OtherBodyIndex :type Integer) (bFromSweep :type Boolean) (SweepResult :type "HitResult Structure (by ref)"))
  (`/Engine/EditorBlueprintResources/ActorMacros.Switch Has Authority`
    (:`Authority`
      (`/Engine/EditorBlueprintResources/StandardMacros.DoOnce` false :!label _label
        (:`Completed`
          (bind _asbp_base_vehicle_parent (cast `/Game/TrafficSystem/BP_BaseVehicleParent` OtherActor))
          (set `self.Ref_Vehicle` _asbp_base_vehicle_parent)
          (bind _returnvalue (`KismetSystemLibrary.K2_SetTimer` null "CheckVehicle" 0.1 true))
          (set `self.Timer` _returnvalue))))))

(event `self.CollisionComponent.OnComponentEndOverlap`
  (params (OverlappedComponent :type "PrimitiveComponent Object Reference") (OtherActor :type "Actor Object Reference") (OtherComp :type "PrimitiveComponent Object Reference") (OtherBodyIndex :type Integer))
  (`/Engine/EditorBlueprintResources/ActorMacros.Switch Has Authority`
    (:`Authority`
      (`|ExecutionSequence`
        (:`then_0`
          (goto _label :!via `Reset`))
        (:`then_1`
          (set `/Game/TrafficSystem/BP_AIVehicleController.CanEnterHighway` true (`/Game/TrafficSystem/BP_BaseVehicleParent.Ref_AiController` (`self.Ref_Vehicle`)))
          (`KismetSystemLibrary.K2_ClearAndInvalidateTimerHandle` (`self.Timer`)))))))

(fn `UserConstructionScript`)