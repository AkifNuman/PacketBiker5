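; Player controller for PacketBiker that spawns the player's character and motor when play begins.
; BeginPlay polls the game instance's Flag, retrying every second while it is zero.
; It then spawns the game instance's Char class at the first PlayerStart found and has player controller 0 possess it.
; The game instance's Motor class spawns separately at a hardcoded transform.
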(event `self.ReceiveBeginPlay`
  (bind _aspacket_biker_game_instance (cast `/Game/Blueprints/PacketBikerGameInstance` (`GameplayStatics.GetGameInstance`) :!label _label))
  (if (== (`/Game/Blueprints/PacketBikerGameInstance.Flag` _aspacket_biker_game_instance) 0)
    (`KismetSystemLibrary.Delay` 1.0)
    (goto _label)
    (else
      (bind _outactors (`GameplayStatics.GetAllActorsOfClass` "/Script/Engine.PlayerStart"))
      (bind (_returnvalue_location _returnvalue_rotation) (`KismetMathLibrary.BreakTransform` (`self.GetTransform` (`|GetArrayItem` _outactors))))
      (bind _returnvalue (`|SpawnActorFromClass` (`/Game/Blueprints/PacketBikerGameInstance.Char` _aspacket_biker_game_instance) (`KismetMathLibrary.MakeTransform` _returnvalue_location _returnvalue_rotation) "Undefined" "OverrideRootScale" null null))
      (`self.Possess` (`GameplayStatics.GetPlayerController` 0) _returnvalue)
      (`|SpawnActorFromClass` (`/Game/Blueprints/PacketBikerGameInstance.Motor` _aspacket_biker_game_instance) (`KismetMathLibrary.MakeTransform` (810.917705 -1305.354756 77.197491) (struct :`Yaw` -270.0)) "Undefined" "OverrideRootScale" null null))))

(fn `UserConstructionScript`)