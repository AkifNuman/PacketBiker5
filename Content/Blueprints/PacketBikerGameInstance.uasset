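; PacketBikerGameInstance is the Game Instance that holds the player's Dolar balance and handles saving and loading progress by slot name.
; SaveGame loads or creates a BP_SaveGame, copies in Dolar, motorcycle fuel and the day counter, then writes the slot inside nested actor loops.
; Therefore, nothing is written unless both a motorcycle and a BP_DayEndigCounter exist.
; LoadGame restores those values to itself and the level actors, with debug prints.
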(fn `LoadGame`
  (params (`Slot Name` :type String))
  (`KismetSystemLibrary.PrintString` "LOADLADIM" true true (struct :`G` 0.66 :`B` 1.0 :`A` 1.0) 4.0)
  (bind _returnvalue (`GameplayStatics.DoesSaveGameExist` `Slot Name`))
  (`KismetSystemLibrary.PrintString` (`KismetStringLibrary.Conv_BoolToString` _returnvalue) true true (struct :`G` 0.66 :`B` 1.0 :`A` 1.0) 10.0)
  (if _returnvalue
    (bind _returnvalue_2 (`GameplayStatics.LoadGameFromSlot` (`local.Slot Name`)))
    (bind _asbp_save_game (cast `/Game/Level_Database/BP_SaveGame` _returnvalue_2))
    (set `self.Dolar` (`/Game/Level_Database/BP_SaveGame.DolarTempo` _asbp_save_game))
    (bind _aspacket_biker_game_instance (cast `/Game/Blueprints/PacketBikerGameInstance` (`GameplayStatics.GetGameInstance`)))
    (bind _output_get (set `self.Dolar` (`/Game/Blueprints/PacketBikerGameInstance.Dolar` _aspacket_biker_game_instance)))
    (`KismetSystemLibrary.PrintString` (`KismetStringLibrary.Conv_IntToString` _output_get) true true (struct :`G` 0.66 :`B` 1.0 :`A` 1.0) 24.0)
    (bind _outactors (`GameplayStatics.GetAllActorsOfClass` "/Game/Vehicles/Motorcycles/BP_BaseMotorcycle.BP_BaseMotorcycle_C"))
    (for _array_element _outactors
      (set `/Game/Vehicles/Motorcycles/BP_BaseMotorcycle.Fuel` (`/Game/Level_Database/BP_SaveGame.FuelTempo` _asbp_save_game) _array_element)
      (bind _outactors_2 (`GameplayStatics.GetAllActorsOfClass` "/Game/Level_Database/DayEndingCounter/BP_DayEndigCounter.BP_DayEndigCounter_C"))
      (for _array_element_2 _outactors_2
        (set `/Game/Level_Database/DayEndingCounter/BP_DayEndigCounter.DayCounter` (`/Game/Level_Database/BP_SaveGame.DayCount` _asbp_save_game) _array_element_2)))
    (else
      (bind _aspacket_biker_game_instance_2 (cast `/Game/Blueprints/PacketBikerGameInstance` (`GameplayStatics.GetGameInstance`)))
      (bind _output_get_2 (set `self.Dolar` (`/Game/Blueprints/PacketBikerGameInstance.Dolar` _aspacket_biker_game_instance_2)))
      (`KismetSystemLibrary.PrintString` (`KismetStringLibrary.Conv_IntToString` _output_get_2) true true (struct :`G` 0.66 :`B` 1.0 :`A` 1.0) 24.0))))

(fn `SaveGame`
  (params (`Slot Name` :type String))
  (bind _returnvalue (`GameplayStatics.DoesSaveGameExist` `Slot Name`))
  (if _returnvalue
    (bind _returnvalue_2 (`GameplayStatics.LoadGameFromSlot` (`local.Slot Name`)))
    (set `self.SaveR` _returnvalue_2)
    (else
      (bind _returnvalue_3 (`GameplayStatics.CreateSaveGameObject` "/Game/Level_Database/BP_SaveGame.BP_SaveGame_C"))
      (bind _output_get (set `self.SaveR` _returnvalue_3))))
  (bind _asbp_save_game (cast `/Game/Level_Database/BP_SaveGame` _output_get))
  (bind _output_get_2 (set `/Game/Level_Database/BP_SaveGame.DolarTempo` (`self.Dolar`) _asbp_save_game))
  (`KismetSystemLibrary.PrintString` (`KismetStringLibrary.Conv_IntToString` _output_get_2))
  (bind _outactors (`GameplayStatics.GetAllActorsOfClass` "/Game/Vehicles/Motorcycles/BP_BaseMotorcycle.BP_BaseMotorcycle_C"))
  (for _array_element _outactors
    (set `/Game/Level_Database/BP_SaveGame.FuelTempo` (`/Game/Vehicles/Motorcycles/BP_BaseMotorcycle.Fuel` _array_element) _asbp_save_game)
    (bind _outactors_2 (`GameplayStatics.GetAllActorsOfClass` "/Game/Level_Database/DayEndingCounter/BP_DayEndigCounter.BP_DayEndigCounter_C"))
    (for _array_element_2 _outactors_2
      (set `/Game/Level_Database/BP_SaveGame.DayCount` (`/Game/Level_Database/DayEndingCounter/BP_DayEndigCounter.DayCounter` _array_element_2) _asbp_save_game)
      (bind _aspacket_biker_game_instance (cast `/Game/Blueprints/PacketBikerGameInstance` (`GameplayStatics.GetGameInstance`)))
      (set `/Game/Blueprints/PacketBikerGameInstance.Dolar` (`self.Dolar`) _aspacket_biker_game_instance)
      (`GameplayStatics.SaveGameToSlot` (`self.SaveR`) (`local.Slot Name`)))))