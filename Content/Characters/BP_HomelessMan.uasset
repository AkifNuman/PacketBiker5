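; BP_HomelessMan is a homeless-man character that can punch and board a scooter.
; The punch event plays a one-shot hook animation, then restores the Animation Blueprint after a delay, while PunchBox overlaps toggle a Punch flag.
; Pressing F while InBox loops over every BP_BaseMotorcycle, hiding the mesh, passing the hobo mesh and anim classes to GetInVehicle, possessing the bike and disabling character collision.
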(event `HomelessPunch`
  (`SkeletalMeshComponent.PlayAnimation` (`self.Mesh`) "/Game/Characters/MainCharacters/Animations/fCityCharsChars/JustChar/Hook_Punch.Hook_Punch" false)
  (`KismetSystemLibrary.Delay` 2.1774)
  (`SkeletalMeshComponent.SetAnimationMode` (`self.Mesh`) "AnimationBlueprint"))

(event `Key|F`
  (params (Key :type "Key Structure"))
  (:`Pressed`
    (`self.ScooterGet_SamWar`)))

(event `self.PunchBox.OnComponentBeginOverlap`
  (params (OverlappedComponent :type "PrimitiveComponent Object Reference") (OtherActor :type "Actor Object Reference") (OtherComp :type "PrimitiveComponent Object Reference") (OtherBodyIndex :type Integer) (bFromSweep :type Boolean) (SweepResult :type "HitResult Structure (by ref)"))
  (set `self.Punch` true))

(event `self.PunchBox.OnComponentEndOverlap`
  (params (OverlappedComponent :type "PrimitiveComponent Object Reference") (OtherActor :type "Actor Object Reference") (OtherComp :type "PrimitiveComponent Object Reference") (OtherBodyIndex :type Integer))
  (set `self.Punch` false))

(fn `ScooterGet_SamWar`
  (if (`self.InBox`)
    (bind _outactors (`GameplayStatics.GetAllActorsOfClass` "/Game/Vehicles/Motorcycles/BP_BaseMotorcycle.BP_BaseMotorcycle_C"))
    (for _array_element _outactors
      (set `/Game/Vehicles/Motorcycles/BP_BaseMotorcycle.InVehicle` true _array_element)
      (bind _asbp_homeless_man (cast `/Game/Characters/BP_HomelessMan` (`GameplayStatics.GetPlayerPawn` 0)))
      (`SceneComponent.SetVisibility` (`self.Mesh`) false false)
      (`/Game/Vehicles/Motorcycles/BP_BaseMotorcycle.GetInVehicle` _array_element "/Game/PolygonCityChar/Characters/SK_Character_Hobo.SK_Character_Hobo" "/Game/Characters/MainCharacters/Animations/fCityCharsChars/CityCharacterAnimBP.CityCharacterAnimBP_C" _asbp_homeless_man "/Game/Characters/MainCharacters/Animations/fCityCharsChars/JustChar/CityCharMovementAnimBP.CityCharMovementAnimBP_C" false false false false false false true false)
      (`Controller.Possess` (`GameplayStatics.GetPlayerController` 0) _array_element)
      (set `self.InBoxPressed` false)
      (`self.SetActorEnableCollision` false))))

(fn `UserConstructionScript`
  (`parent.UserConstructionScript`))