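; Player character Blueprint for the rich female sci-fi character, with scooter entry, a punch and a ragdoll function.
; F, while InBox is set, loops over all BP_BaseMotorcycle actors, hiding the mesh, passing character assets to GetInVehicle, possessing each, disabling collision and adding fuel and scooter widgets.
; Right mouse plays a punch animation, then restores AnimBP mode after a delay; PunchBox overlaps toggle the Punch flag.
; Ragdoll enables mesh physics simulation.
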(event `Key|F`
  (params (Key :type "Key Structure"))
  (:`Pressed`
    (`self.ScooterGet_RichFemSci-Fi`)))

(event `Key|RightMouseButton`
  (params (Key :type "Key Structure"))
  (:`Pressed`
    (`SkeletalMeshComponent.PlayAnimation` (`self.Mesh`) "/Game/Characters/MainCharacters/Animations/fSci-fiChars/JustChar/Hook_Punch.Hook_Punch" false)
    (`KismetSystemLibrary.Delay` 2.1774)
    (`SkeletalMeshComponent.SetAnimationMode` (`self.Mesh`) "AnimationBlueprint")))

(event `self.PunchBox.OnComponentBeginOverlap`
  (params (OverlappedComponent :type "PrimitiveComponent Object Reference") (OtherActor :type "Actor Object Reference") (OtherComp :type "PrimitiveComponent Object Reference") (OtherBodyIndex :type Integer) (bFromSweep :type Boolean) (SweepResult :type "HitResult Structure (by ref)"))
  (set `self.Punch` true))

(event `self.PunchBox.OnComponentEndOverlap`
  (params (OverlappedComponent :type "PrimitiveComponent Object Reference") (OtherActor :type "Actor Object Reference") (OtherComp :type "PrimitiveComponent Object Reference") (OtherBodyIndex :type Integer))
  (set `self.Punch` false))

(fn `Ragdoll_RichFemSci-Fi`
  (`PrimitiveComponent.SetSimulatePhysics` (`self.Mesh`) true))

(fn `ScooterGet_RichFemSci-Fi`
  (if (`self.InBox`)
    (bind _outactors (`GameplayStatics.GetAllActorsOfClass` "/Game/Vehicles/Motorcycles/BP_BaseMotorcycle.BP_BaseMotorcycle_C"))
    (for _array_element _outactors
      (`SceneComponent.SetVisibility` (`self.Mesh`) false false)
      (set `self.InBoxPressed` true)
      (`/Game/Vehicles/Motorcycles/Scooter/Scooter_BP.GetInVehicle` _array_element "/Game/PolygonScifi/Meshes/Characters/SK_Character_Rich_Female_01.SK_Character_Rich_Female_01" "/Game/Characters/MainCharacters/Animations/fSci-fiChars/JustChar/Sci-Fi-CharsMovementAnimBP.Sci-Fi-CharsMovementAnimBP_C" self "/Game/Characters/MainCharacters/Animations/fSci-fiChars/Sci-FiMovementAnimBP.Sci-FiMovementAnimBP_C" false false false false false false false true)
      (`Controller.Possess` (`GameplayStatics.GetPlayerController` 0) _array_element)
      (set `self.InBoxPressed` false)
      (`self.SetActorEnableCollision` false)
      (bind _returnvalue (`|CreateWidget` "/Game/Fuel/WB_FuelBar.WB_FuelBar_C"))
      (`UserWidget.AddToViewport` _returnvalue 0)
      (bind _returnvalue_2 (`|CreateWidget` "/Game/Interfaces/ScooterInterface.ScooterInterface_C"))
      (`UserWidget.AddToViewport` _returnvalue_2 0))))

(fn `UserConstructionScript`
  (`parent.UserConstructionScript`))