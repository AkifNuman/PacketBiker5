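; BP_Grandma is the grandma character, who can mount a scooter when the player presses F inside a trigger box.
; Mounting loops over every BP_BaseMotorcycle, hands it her mesh and anim classes, possesses it, hides her, disables her collision and adds fuel and scooter widgets.
; Other events briefly ragdoll her, temporarily disable post-processing behind a DoOnce, and show a mission counter.
; Random-roam movement is present but disconnected.
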(event `SpecialForceGrandma`
  (bind _postprocess (`self.PostProcess`))
  (`/Engine/EditorBlueprintResources/StandardMacros.DoOnce` false :!label _label
    (:`Completed`
      (`KismetSystemLibrary.PrintString` "Hello")
      (set `PostProcessComponent.bEnabled` false _postprocess)
      (`KismetSystemLibrary.Delay` 10.0)
      (set `PostProcessComponent.bEnabled` true _postprocess)
      (`KismetSystemLibrary.Delay` 5.0)
      (goto _label :!via `Reset`))))

(event `timer`
  (`KismetSystemLibrary.K2_SetTimerDelegate` (delegate `timer`) 0.016667 true)
  (bind _returnvalue (`|CreateWidget` "/Game/Level_Database/WB_MissionCounter.WB_MissionCounter_C"))
  (`UserWidget.AddToViewport` _returnvalue 0))

(event `Random Roam`)

(event `Key|F`
  (params (Key :type "Key Structure"))
  (:`Pressed`
    (`self.ScooterGet_Grandma`)))

(event `Ragdoll_SamWar`
  (bind _mesh (`self.Mesh`))
  (`PrimitiveComponent.SetSimulatePhysics` _mesh true)
  (`KismetSystemLibrary.Delay` 0.7)
  (`PrimitiveComponent.SetSimulatePhysics` _mesh false))

(fn `ScooterGet_Grandma`
  (if (`self.InBox`)
    (bind _outactors (`GameplayStatics.GetAllActorsOfClass` "/Game/Vehicles/Motorcycles/BP_BaseMotorcycle.BP_BaseMotorcycle_C"))
    (for _array_element _outactors
      (set `/Game/Vehicles/Motorcycles/BP_BaseMotorcycle.InVehicle` true _array_element)
      (bind _asbp_grandma (cast `/Game/Characters/BP_Grandma` (`GameplayStatics.GetPlayerPawn` 0)))
      (`SceneComponent.SetVisibility` (`self.Mesh`) false false)
      (`/Game/Vehicles/Motorcycles/BP_BaseMotorcycle.GetInVehicle` _array_element "/Game/PolygonCityChar/Characters/SK_Character_Grandma.SK_Character_Grandma" "/Game/Characters/MainCharacters/Animations/fCityCharsChars/CityCharacterAnimBP.CityCharacterAnimBP_C" _asbp_grandma "/Game/Characters/MainCharacters/Animations/fCityCharsChars/JustChar/CityCharMovementAnimBP.CityCharMovementAnimBP_C" false true false false false false false false)
      (`Controller.Possess` (`GameplayStatics.GetPlayerController` 0) _array_element)
      (set `self.InBoxPressed` false)
      (`self.SetActorEnableCollision` false)
      (bind _returnvalue (`|CreateWidget` "/Game/Fuel/WB_FuelBar.WB_FuelBar_C"))
      (`UserWidget.AddToViewport` _returnvalue 0)
      (bind _returnvalue_2 (`|CreateWidget` "/Game/Interfaces/ScooterInterface.ScooterInterface_C"))
      (`UserWidget.AddToViewport` _returnvalue_2 0))))

(fn `UserConstructionScript`
  (`parent.UserConstructionScript`))