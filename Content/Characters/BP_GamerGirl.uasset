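; BP_GamerGirl is a character Blueprint for the gamer girl, with motorcycle boarding, a punch and a brief ragdoll.
; F, while InBox is set, hides the mesh, disables collision and loops over every BP_BaseMotorcycle, calling GetInVehicle and possessing each in turn.
; SpecialForce toggles a post-process effect, and PunchBox overlaps set the Punch flag.
; Punch and ragdoll events use timed delays to end the montage-free animation or physics simulation.
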(event `InputAction|SpecialForce`
  (params (Key :type "Key Structure"))
  (bind _postprocess (`self.PostProcess`))
  (:`Pressed`
    (`/Engine/EditorBlueprintResources/StandardMacros.FlipFlop`
      (:`A`
        (`SceneComponent.SetVisibility` _postprocess true false))
      (:`B`
        (`SceneComponent.SetVisibility` _postprocess false false)))))

(event `Key|F`
  (params (Key :type "Key Structure"))
  (:`Pressed`
    (`self.ScooterGet_GamerGirl`)))

(event `Ragdoll_GamerGirl`
  (bind _mesh (`self.Mesh`))
  (`PrimitiveComponent.SetSimulatePhysics` _mesh true)
  (`KismetSystemLibrary.Delay` 0.7)
  (`PrimitiveComponent.SetSimulatePhysics` _mesh false))

(event `AnimeGirlPunch`
  (`SkeletalMeshComponent.PlayAnimation` (`self.Mesh`) "/Game/Characters/MainCharacters/Animations/fCityCharsChars/JustChar/Hook_Punch.Hook_Punch" false)
  (`KismetSystemLibrary.Delay` 2.1774)
  (`SkeletalMeshComponent.SetAnimationMode` (`self.Mesh`) "AnimationBlueprint"))

(event `self.PunchBox.OnComponentBeginOverlap`
  (params (OverlappedComponent :type "PrimitiveComponent Object Reference") (OtherActor :type "Actor Object Reference") (OtherComp :type "PrimitiveComponent Object Reference") (OtherBodyIndex :type Integer) (bFromSweep :type Boolean) (SweepResult :type "HitResult Structure (by ref)"))
  (set `self.Punch` true))

(event `self.PunchBox.OnComponentEndOverlap`
  (params (OverlappedComponent :type "PrimitiveComponent Object Reference") (OtherActor :type "Actor Object Reference") (OtherComp :type "PrimitiveComponent Object Reference") (OtherBodyIndex :type Integer))
  (set `self.Punch` false))

(fn `ScooterGet_GamerGirl`
  (if (`self.InBox`)
    (bind _outactors (`GameplayStatics.GetAllActorsOfClass` "/Game/Vehicles/Motorcycles/BP_BaseMotorcycle.BP_BaseMotorcycle_C"))
    (for _array_element _outactors
      (`SceneComponent.SetVisibility` (`self.Mesh`) false false)
      (set `self.InBoxPressed` true)
      (`/Game/Vehicles/Motorcycles/Scooter/Scooter_BP.GetInVehicle` _array_element "/Game/PolygonCityChar/Characters/SK_Character_GamerGirl.SK_Character_GamerGirl" "/Game/Characters/MainCharacters/Animations/fCityCharsChars/CityCharacterAnimBP.CityCharacterAnimBP_C" self "/Game/Characters/MainCharacters/Animations/fCityCharsChars/JustChar/CityCharMovementAnimBP.CityCharMovementAnimBP_C" false false false true false false false false)
      (`self.SetActorEnableCollision` false)
      (`Controller.Possess` (`GameplayStatics.GetPlayerController` 0) _array_element)
      (set `self.InBoxPressed` false))))

(fn `UserConstructionScript`
  (`parent.UserConstructionScript`))