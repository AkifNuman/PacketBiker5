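; BP_Grandpa is the Grandpa character, with a slow-motion ability, a hook punch and motorcycle boarding.
; A self-rescheduling timer with a Delay charges TimeStop over about a minute; R then briefly slows the world while speeding Grandpa up.
; GrandpaPunch plays the hook animation, while PunchBox overlaps toggle a Punch flag.
; F, when InBox, hides the mesh, calls GetInVehicle on every BP_BaseMotorcycle and possesses each in turn.
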(event `Key|R`
  (params (Key :type "Key Structure"))
  (:`Pressed`
    (if (`self.isTimeStop`)
      (`GameplayStatics.SetGlobalTimeDilation` 0.3)
      (set `self.CustomTimeDilation` 4.0)
      (set `self.isTimeStop` false)
      (`KismetSystemLibrary.Delay` 5.0)
      (`GameplayStatics.SetGlobalTimeDilation` 1.0)
      (set `self.CustomTimeDilation` 1.0)
      (set `self.Time` 0))))

(event `TimeStop`
  (`KismetSystemLibrary.K2_SetTimerDelegate` (delegate `TimeStop`) 0.033333)
  (`KismetSystemLibrary.Delay` 1.0)
  (bind _output_get (set `self.Time` (+ (`self.Time`) 1)))
  (if (>= _output_get 60)
    (set `self.isTimeStop` true)))

(event `self.ReceiveBeginPlay`
  (`parent.ReceiveBeginPlay`)
  (`self.TimeStop`))

(event `GrandpaPunch`
  (`SkeletalMeshComponent.PlayAnimation` (`self.Mesh`) "/Game/Characters/MainCharacters/Animations/fCityCharsChars/JustChar/Hook_Punch.Hook_Punch" false)
  (`KismetSystemLibrary.Delay` 2.1774)
  (`SkeletalMeshComponent.SetAnimationMode` (`self.Mesh`) "AnimationBlueprint"))

(event `self.PunchBox.OnComponentBeginOverlap`
  (params (OverlappedComponent :type "PrimitiveComponent Object Reference") (OtherActor :type "Actor Object Reference") (OtherComp :type "PrimitiveComponent Object Reference") (OtherBodyIndex :type Integer) (bFromSweep :type Boolean) (SweepResult :type "HitResult Structure (by ref)"))
  (set `self.Punch` true))

(event `self.PunchBox.OnComponentEndOverlap`
  (params (OverlappedComponent :type "PrimitiveComponent Object Reference") (OtherActor :type "Actor Object Reference") (OtherComp :type "PrimitiveComponent Object Reference") (OtherBodyIndex :type Integer))
  (set `self.Punch` false))

(event `Key|F`
  (params (Key :type "Key Structure"))
  (:`Pressed`
    (`self.ScooterGet_SamWar`)))

(fn `ScooterGet_SamWar`
  (if (`self.InBox`)
    (bind _outactors (`GameplayStatics.GetAllActorsOfClass` "/Game/Vehicles/Motorcycles/BP_BaseMotorcycle.BP_BaseMotorcycle_C"))
    (for _array_element _outactors
      (bind _asbp_grandpa (cast `/Game/Characters/BP_Grandpa` (`GameplayStatics.GetPlayerPawn` 0)))
      (`SceneComponent.SetVisibility` (`self.Mesh`) false false)
      (`/Game/Vehicles/Motorcycles/BP_BaseMotorcycle.GetInVehicle` _array_element "/Game/PolygonCityChar/Characters/SK_Character_Grandpa.SK_Character_Grandpa" "/Game/Characters/MainCharacters/Animations/fCityCharsChars/CityCharacterAnimBP.CityCharacterAnimBP_C" _asbp_grandpa "/Game/Characters/MainCharacters/Animations/fCityCharsChars/JustChar/CityCharMovementAnimBP.CityCharMovementAnimBP_C" false false false false false true false false)
      (`Controller.Possess` (`GameplayStatics.GetPlayerController` 0) _array_element)
      (set `self.InBoxPressed` false)
      (`self.SetActorEnableCollision` false))))

(fn `UserConstructionScript`
  (`parent.UserConstructionScript`))