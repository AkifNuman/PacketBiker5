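; Fuel location marker actor that displays its distance in meters through its Icon widget and hides itself within about 4 meters.
; A looping timer started at BeginPlay re-runs LocMarker roughly 30 times a second, measuring from the player character.
; When no valid player character exists, it loops over every BP_BaseMotorcycle instead, so the last one iterated sets the final visibility and distance text.
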(event `self.ReceiveBeginPlay`
  (`self.LocMarker`))

(event `LocMarker`
  (bind _returnvalue (`GameplayStatics.GetPlayerCharacter` 0))
  (bind _returnvalue_2 (`KismetMathLibrary.FTrunc` (/ (`KismetMathLibrary.Vector_Distance` (`self.K2_GetActorLocation` _returnvalue) (`self.K2_GetActorLocation`)) 100.0)))
  (`KismetSystemLibrary.K2_SetTimerDelegate` (delegate `LocMarker`) 0.033333 true)
  (`/Engine/EditorBlueprintResources/StandardMacros.IsValid` _returnvalue
    (:`Is Valid`
      (if (<= _returnvalue_2 4)
        (`self.SetActorHiddenInGame` true)
        (else
          (`self.SetActorHiddenInGame` false)))
      (message `/Game/Map/LocationMarker/BPI_MarkerWidget.UpdateDistance` (`WidgetComponent.GetUserWidgetObject` (`self.Icon`)) (`KismetTextLibrary.Conv_StringToText` (`KismetStringLibrary.Concat_StrStr` (`KismetTextLibrary.Conv_TextToString` (`KismetTextLibrary.Conv_IntToText` _returnvalue_2)) "m"))))
    (:`Is Not Valid`
      (bind _outactors (`GameplayStatics.GetAllActorsOfClass` "/Game/Vehicles/Motorcycles/BP_BaseMotorcycle.BP_BaseMotorcycle_C"))
      (for _array_element _outactors
        (bind _returnvalue_3 (`KismetMathLibrary.FTrunc` (/ (`KismetMathLibrary.Vector_Distance` (`self.K2_GetActorLocation` _array_element) (`self.K2_GetActorLocation`)) 100.0)))
        (if (<= _returnvalue_3 4)
          (`self.SetActorHiddenInGame` true)
          (else
            (`self.SetActorHiddenInGame` false)))
        (message `/Game/Map/LocationMarker/BPI_MarkerWidget.UpdateDistance` (`WidgetComponent.GetUserWidgetObject` (`self.Icon`)) (`KismetTextLibrary.Conv_StringToText` (`KismetStringLibrary.Concat_StrStr` (`KismetTextLibrary.Conv_TextToString` (`KismetTextLibrary.Conv_IntToText` _returnvalue_3)) "m")))))))

(fn `UserConstructionScript`)