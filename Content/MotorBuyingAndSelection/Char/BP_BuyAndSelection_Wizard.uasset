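; BP_BuyAndSelection_Wizard is the Wizard actor in the motor buying and selection area, showing its details UI when something enters its trigger box.
; Box begin overlap creates the WB_WizardDetails widget and adds it to the viewport.
; End overlap removes all widgets, then recreates the WB_DolarInstance and Wb_SettingButton widgets to restore that UI.
; Neither overlap event checks which actor triggered it.
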(event `self.Box.OnComponentBeginOverlap`
  (params (OverlappedComponent :type "PrimitiveComponent Object Reference") (OtherActor :type "Actor Object Reference") (OtherComp :type "PrimitiveComponent Object Reference") (OtherBodyIndex :type Integer) (bFromSweep :type Boolean) (SweepResult :type "HitResult Structure (by ref)"))
  (bind _returnvalue (`|CreateWidget` "/Game/MotorBuyingAndSelection/Char/WB_WizardDetails.WB_WizardDetails_C"))
  (`UserWidget.AddToViewport` _returnvalue 0))

(event `self.Box.OnComponentEndOverlap`
  (params (OverlappedComponent :type "PrimitiveComponent Object Reference") (OtherActor :type "Actor Object Reference") (OtherComp :type "PrimitiveComponent Object Reference") (OtherBodyIndex :type Integer))
  (`WidgetLayoutLibrary.RemoveAllWidgets`)
  (bind _returnvalue (`|CreateWidget` "/Game/Level_Database/WB_DolarInstance.WB_DolarInstance_C"))
  (`UserWidget.AddToViewport` _returnvalue 0)
  (bind _returnvalue_2 (`|CreateWidget` "/Game/Interfaces/Wb_SettingButton_Auto2.Wb_SettingButton_C"))
  (`UserWidget.AddToViewport` _returnvalue_2 0))

(fn `UserConstructionScript`
  (`parent.UserConstructionScript`))