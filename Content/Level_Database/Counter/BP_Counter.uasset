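; BP_Counter is a countdown actor that fails a timed box-delivery mission when time runs out.
; On BeginPlay it shows WB_MissionCounter and starts a one-second timer event that decrements MissionCounter and plays a tick sound.
; At zero, if a BP_TargetCalculator exists, nested GetAllActorsOfClass loops deduct money, clear the counter flag, hide boxes and points, remove markers and widget, then destroy the counter.
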(event `self.ReceiveBeginPlay`
  (`|ExecutionSequence`
    (:`then_0`
      (`self.Is Mission Complete`))
    (:`then_1`
      (bind _returnvalue (`|CreateWidget` "/Game/Level_Database/WB_MissionCounter.WB_MissionCounter_C" (`GameplayStatics.GetPlayerController` 0)))
      (`UserWidget.AddToViewport` _returnvalue 0))))

(event `Is Mission Complete`
  (`KismetSystemLibrary.K2_SetTimerDelegate` (delegate `Is Mission Complete`) 1.0 true)
  (set `self.MissionCounter` (- (`self.MissionCounter`) 1))
  (`GameplayStatics.PlaySoundAtLocation` "/Game/PacketBikerAudio/MissionSound/clocky.clocky" (`self.K2_GetActorLocation` (`GameplayStatics.GetPlayerPawn` 0)) (struct) 1.0 1.0 0.0 null null null null)
  (if (== (`self.MissionCounter`) 0)
    (bind _outactors (`GameplayStatics.GetAllActorsOfClass` "/Game/Mission/BP_TargetCalculator.BP_TargetCalculator_C"))
    (if (`KismetArrayLibrary.Array_IsValidIndex` _outactors)
      (`GameplayStatics.PlaySoundAtLocation` "/Game/PacketBikerAudio/MissionFail/fail.fail" (`self.K2_GetActorLocation` (`GameplayStatics.GetPlayerPawn` 0)) (struct) 1.0 1.0 0.0 null null null null)
      (bind _outactors_2 (`GameplayStatics.GetAllActorsOfClass` "/Game/Level_Database/BP_LevelDatabase.Bp_LevelDatabase_C"))
      (for _array_element _outactors_2
        (set `/Game/Level_Database/BP_LevelDatabase.Dolar` (- (`/Game/Level_Database/BP_LevelDatabase.Dolar` _array_element) 5) _array_element)
        (set `/Game/Level_Database/BP_LevelDatabase.isCounter` false _array_element)
        (bind _outactors_3 (`GameplayStatics.GetAllActorsOfClass` "/Game/Vehicles/Motorcycles/BP_BaseMotorcycle.BP_BaseMotorcycle_C"))
        (for _array_element_2 _outactors_3
          (`SceneComponent.SetVisibility` (`/Game/Vehicles/Motorcycles/BP_BaseMotorcycle.StaticBox` _array_element_2) false false)
          (bind _outactors_4 (`GameplayStatics.GetAllActorsOfClass` "/Game/Characters/BP_Character.BP_Character_C"))
          (for _array_element_3 _outactors_4
            (set `/Game/Characters/BP_Character.HasBox` false _array_element_3)
            (`SceneComponent.SetVisibility` (`/Game/Characters/BP_Character.TasimaKutusu` _array_element_3) false false)
            (bind _outactors_5 (`GameplayStatics.GetAllActorsOfClass` "/Game/Map/LocationMarker/BP_LocationMarkerRes.BP_LocationMarkerRes_C"))
            (for _array_element_4 _outactors_5
              (`self.K2_DestroyActor` _array_element_4)
              (bind _outactors_6 (`GameplayStatics.GetAllActorsOfClass` "/Game/Mission/BP_TargetCalculator.BP_TargetCalculator_C"))
              (for _array_element_5 _outactors_6
                (`self.K2_DestroyActor` _array_element_5)
                (bind _foundwidgets (`WidgetBlueprintLibrary.GetAllWidgetsOfClass` "/Game/Level_Database/WB_MissionCounter.WB_MissionCounter_C"))
                (for _array_element_6 _foundwidgets
                  (`Widget.RemoveFromParent` _array_element_6)
                  (bind _outactors_7 (`GameplayStatics.GetAllActorsOfClass` "/Game/Mission/BP_TargetPoint.BP_TargetPoint_C"))
                  (for _array_element_7 _outactors_7
                    (`self.SetActorHiddenInGame` _array_element_7 true)
                    (bind _outactors_8 (`GameplayStatics.GetAllActorsOfClass` "/Game/Mission/BP_RestaurantPoint.BP_RestaurantPoint_C"))
                    (for _array_element_8 _outactors_8
                      (`self.SetActorHiddenInGame` _array_element_8 true)
                      (`self.K2_DestroyActor`))))))))))))

(fn `UserConstructionScript`)