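; Level manager for the biker game that persists player economy and offers new target jobs.
; SaveGame and LoadGame move money, expenses, motorcycle fuel and day count through BP_SaveGame, though the GameInstance's money overrides the saved value on load.
; BeginPlay loads Slot1, then loops: with no BP_TargetCalculator present, it shows a notification after a random delay and polls the Phone widget, spawning one on accept.
; The dash collectable UI logic is disconnected.
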(event `self.ReceiveBeginPlay`
  (`|ExecutionSequence`
    (:`then_0`
      (`self.LoadGame` "Slot1"))
    (:`then_1`
      (`self.Spawn target calculator`))
    (:`then_2`
      (`self.DashCollecCount`))))

(event `Spawn target calculator`
  (bind _outactors (`GameplayStatics.GetAllActorsOfClass` "/Game/Mission/BP_TargetCalculator.BP_TargetCalculator_C" :!label _label))
  (if (`KismetArrayLibrary.Array_IsValidIndex` _outactors)
    (`KismetSystemLibrary.Delay` 20.0)
    (goto _label)
    (else
      (`KismetSystemLibrary.Delay` (`KismetMathLibrary.Conv_IntToDouble` (`KismetMathLibrary.RandomIntegerInRange` 7 13)))
      (`GameplayStatics.PlaySoundAtLocation` "/Game/PacketBikerAudio/Notification/notifications-sound-127856.notifications-sound-127856" (`self.K2_GetActorLocation`) (struct) 1.0 1.0 0.0 null null null null)
      (bind _returnvalue (`|CreateWidget` "/Game/Mission/WB_Notif.WB_Notif_C"))
      (`UserWidget.AddToViewport` _returnvalue 0)
      (bind _foundwidgets (`WidgetBlueprintLibrary.GetAllWidgetsOfClass` "/Game/Mission/Phone.Phone_C" :!label _label_2))
      (for _array_element _foundwidgets
        (if (`/Game/Mission/Phone.pressed accept` _array_element)
          (`|SpawnActorFromClass` "/Game/Mission/BP_TargetCalculator.BP_TargetCalculator_C" (`self.GetTransform` (`GameplayStatics.GetPlayerController` 0)) "AlwaysSpawn" "OverrideRootScale" null null)
          (set `self.isCounter` true)
          (set `/Game/Mission/Phone.pressed accept` false _array_element)
          (goto _label)
          (elif (`/Game/Mission/Phone.pressed decline` _array_element)
            (set `/Game/Mission/Phone.pressed decline` false _array_element)
            (goto _label)
            (else
              (`KismetSystemLibrary.Delay` 0.2)
              (goto _label_2))))))))

(event `DashCollecCount`)

(fn `LoadGame`
  (params (`Slot Name` :type String))
  (`KismetSystemLibrary.PrintString` "LOADLADIM" true true (struct :`G` 0.66 :`B` 1.0 :`A` 1.0) 4.0)
  (bind _returnvalue (`GameplayStatics.DoesSaveGameExist` `Slot Name`))
  (`KismetSystemLibrary.PrintString` (`KismetStringLibrary.Conv_BoolToString` _returnvalue) true true (struct :`G` 0.66 :`B` 1.0 :`A` 1.0) 10.0)
  (if _returnvalue
    (bind _returnvalue_2 (`GameplayStatics.LoadGameFromSlot` (`local.Slot Name`)))
    (bind _asbp_save_game (cast `/Game/Level_Database/BP_SaveGame` _returnvalue_2))
    (set `self.Dolar` (`/Game/Level_Database/BP_SaveGame.DolarTempo` _asbp_save_game))
    (set `self.Rent` (`/Game/Level_Database/BP_SaveGame.RentTempo` _asbp_save_game))
    (set `self.Food` (`/Game/Level_Database/BP_SaveGame.FoodTempo` _asbp_save_game))
    (set `self.Heat` (`/Game/Level_Database/BP_SaveGame.HeatTempo` _asbp_save_game))
    (bind _aspacket_biker_game_instance (cast `/Game/Blueprints/PacketBikerGameInstance` (`GameplayStatics.GetGameInstance`)))
    (bind _output_get (set `self.Dolar` (`/Game/Blueprints/PacketBikerGameInstance.Dolar` _aspacket_biker_game_instance)))
    (`KismetSystemLibrary.PrintString` (`KismetStringLibrary.Conv_IntToString` _output_get) true true (struct :`G` 0.66 :`B` 1.0 :`A` 1.0) 24.0)
    (bind _outactors (`GameplayStatics.GetAllActorsOfClass` "/Game/Vehicles/Motorcycles/BP_BaseMotorcycle.BP_BaseMotorcycle_C"))
    (for _array_element _outactors
      (set `/Game/Vehicles/Motorcycles/BP_BaseMotorcycle.Fuel` (`/Game/Level_Database/BP_SaveGame.FuelTempo` _asbp_save_game) _array_element)
      (bind _outactors_2 (`GameplayStatics.GetAllActorsOfClass` "/Game/Level_Database/DayEndingCounter/BP_DayEndigCounter.BP_DayEndigCounter_C"))
      (for _array_element_2 _outactors_2
        (set `/Game/Level_Database/DayEndingCounter/BP_DayEndigCounter.DayCounter` (`/Game/Level_Database/BP_SaveGame.DayCount` _asbp_save_game) _array_element_2)))
    (else
      (bind _aspacket_biker_game_instance_2 (cast `/Game/Blueprints/PacketBikerGameInstance` (`GameplayStatics.GetGameInstance`)))
      (bind _output_get_2 (set `self.Dolar` (`/Game/Blueprints/PacketBikerGameInstance.Dolar` _aspacket_biker_game_instance_2)))
      (`KismetSystemLibrary.PrintString` (`KismetStringLibrary.Conv_IntToString` _output_get_2) true true (struct :`G` 0.66 :`B` 1.0 :`A` 1.0) 24.0))))

(fn `SaveGame`
  (params (`Slot Name` :type String))
  (bind _returnvalue (`GameplayStatics.DoesSaveGameExist` `Slot Name`))
  (if _returnvalue
    (bind _returnvalue_2 (`GameplayStatics.LoadGameFromSlot` (`local.Slot Name`)))
    (set `self.SaveRef` _returnvalue_2)
    (else
      (bind _returnvalue_3 (`GameplayStatics.CreateSaveGameObject` "/Game/Level_Database/BP_SaveGame.BP_SaveGame_C"))
      (bind _output_get (set `self.SaveRef` _returnvalue_3))))
  (bind _asbp_save_game (cast `/Game/Level_Database/BP_SaveGame` _output_get))
  (bind _output_get_2 (set `/Game/Level_Database/BP_SaveGame.DolarTempo` (`self.Dolar`) _asbp_save_game))
  (`KismetSystemLibrary.PrintString` (`KismetStringLibrary.Conv_IntToString` _output_get_2))
  (set `/Game/Level_Database/BP_SaveGame.HeatTempo` (`self.Heat`) _asbp_save_game)
  (set `/Game/Level_Database/BP_SaveGame.RentTempo` (`self.Rent`) _asbp_save_game)
  (set `/Game/Level_Database/BP_SaveGame.FoodTempo` (`self.Food`) _asbp_save_game)
  (bind _outactors (`GameplayStatics.GetAllActorsOfClass` "/Game/Vehicles/Motorcycles/BP_BaseMotorcycle.BP_BaseMotorcycle_C"))
  (for _array_element _outactors
    (set `/Game/Level_Database/BP_SaveGame.FuelTempo` (`/Game/Vehicles/Motorcycles/BP_BaseMotorcycle.Fuel` _array_element) _asbp_save_game)
    (bind _outactors_2 (`GameplayStatics.GetAllActorsOfClass` "/Game/Level_Database/DayEndingCounter/BP_DayEndigCounter.BP_DayEndigCounter_C"))
    (for _array_element_2 _outactors_2
      (set `/Game/Level_Database/BP_SaveGame.DayCount` (`/Game/Level_Database/DayEndingCounter/BP_DayEndigCounter.DayCounter` _array_element_2) _asbp_save_game)
      (bind _aspacket_biker_game_instance (cast `/Game/Blueprints/PacketBikerGameInstance` (`GameplayStatics.GetGameInstance`)))
      (set `/Game/Blueprints/PacketBikerGameInstance.Dolar` (`self.Dolar`) _aspacket_biker_game_instance)
      (`GameplayStatics.SaveGameToSlot` (`self.SaveRef`) (`local.Slot Name`)))))

(fn `UserConstructionScript`)