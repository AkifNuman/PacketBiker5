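; BP_DayEndigCounter is an actor that counts time toward the end of each in-game day.
; From BeginPlay, DayCount re-fires itself on a fast looping timer, while a one-second Delay limits DayEndCounter increments to roughly one per second.
; At MaxDayEnd it increments DayCounter, resets the count, clears all widgets, pauses the game and shows the WB_DayEnding screen.
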(event `self.ReceiveBeginPlay`
  (`self.DayCount`))

(event `DayCount`
  (`KismetSystemLibrary.K2_SetTimerDelegate` (delegate `DayCount`) 0.033333 true)
  (`KismetSystemLibrary.Delay` 1.0)
  (set `self.DayEndCounter` (+ (`self.DayEndCounter`) 1))
  (if (== (`self.DayEndCounter`) (`self.MaxDayEnd`))
    (`KismetSystemLibrary.PrintString` "Hello")
    (set `self.DayCounter` (+ (`self.DayCounter`) 1))
    (set `self.DayEndCounter` 0)
    (`WidgetLayoutLibrary.RemoveAllWidgets`)
    (`GameplayStatics.SetGamePaused` true)
    (bind _returnvalue (`|CreateWidget` "/Game/Level_Database/WB_DayEnding.WB_DayEnding_C" (`GameplayStatics.GetPlayerController` 0)))
    (`UserWidget.AddToViewport` _returnvalue 0)))

(fn `UserConstructionScript`)